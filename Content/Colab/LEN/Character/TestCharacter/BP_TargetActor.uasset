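; BP_TargetActor is an actor that flies out to a target point and then returns to its owner (the player), boomerang-style.
; SetMove places it at a start location and stores the destination.
; Tick runs an IsMove state machine: constant-speed interpolation to the target, then back to the owner's live location, then idle on arrival.
; Moves are non-swept and the actor is not destroyed on return.
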(event Custom|SetMove
  (params (TargetLocation :type Vector) (StartLocation :type Vector))
  (Variables|Default|SetTargetLocation TargetLocation)
  (bind _output_get (Variables|Default|SetStartLocation StartLocation))
  (bind _returnvalue (Transformation|SetActorLocation _output_get false false))
  (if _returnvalue
    (Variables|Default|SetIsMove 1)))

(event EventTick
  (params (DeltaSeconds :type Float%20%28single-precision%29))
  (switch int (Variables|Default|GetIsMove)
    (:1
      ;[1 1 1] 목표 지점으로 가기
      (if (< (Math|Vector|Distance(Vector) (Transformation|GetActorLocation) (Variables|Default|GetTargetLocation)) 1.0)
        (Variables|Default|SetIsMove 2)
        (else
          (Transformation|SetActorLocation (Math|Interpolation|VInterptoConstant (Transformation|GetActorLocation) (Variables|Default|GetTargetLocation) DeltaSeconds 1e+03) false false))))
    (:2
      ;[1 1 1] 플레이어(오너)에게 돌아오기
      (bind _myowner (Variables|Default|GetMyOwner)
        (:then
          (Variables|Default|SetTargetLocation (Transformation|GetActorLocation _myowner))
          (if (< (Math|Vector|Distance(Vector) (Transformation|GetActorLocation) (Variables|Default|GetTargetLocation)) 1.0)
            (Variables|Default|SetIsMove 0)
            (else
              (Transformation|SetActorLocation (Math|Interpolation|VInterptoConstant (Transformation|GetActorLocation) (Variables|Default|GetTargetLocation) DeltaSeconds 1e+03) false false))))
        (:else)))))

(event EventBeginPlay
  (Variables|Default|SetMyOwner (Components|GetOwner)))

(fn ConstructionScript)