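; Physics-based Gunner pawn that sets up Enhanced Input for look, move and jump.
; Look drives controller rotation, while movement relative to control yaw and jump requests go to BPMoveableComponentLAN, whose move tick runs only on authority.
; Tick also wakes all skeletal mesh rigid bodies every frame.
; GetHandVelocity exposes hand component velocity and target, and capsule hits on RidingTestDummy print its collision object type for debugging.
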(event OnComponentHit(Capsule)
  (params (HitComponent :type Primitive%20Component%20Object%20Reference) (OtherActor :type Actor%20Object%20Reference) (OtherComp :type Primitive%20Component%20Object%20Reference) (NormalImpulse :type Vector :default "0, 0, 0") (Hit :type Hit%20Result%20Structure%20%28by%20ref%29))
  (bind _asriding_test_dummy (Utilities|Casting|CastToRidingTestDummy OtherActor))
  (Development|PrintString (Utilities|String|EnumtoString (Collision|GetCollisionObjectType (Variables|/Game/Colab/LEN/RidingTestDummy.RidingTestDummy_C|GetStaticMesh _asriding_test_dummy)))))

(event Input|EnhancedActionEvents|EnhancedInputActionIA_GunnerMove
  (params (ActionValue :type Vector%202D%20Structure) (ElapsedSeconds :type Float%20%28double-precision%29) (TriggeredSeconds :type Float%20%28double-precision%29) (InputAction :type Input%20Action%20Object%20Reference :default "/Game/Colab/LEN/GunnerIMC/IA/IA_GunnerMove.IA_GunnerMove"))
  (bind _bp_moveablecomponentlan (Variables|Default|GetBP_MoveableComponentLAN))
  ;[1 1 1] 시야돌리기,이동,점프
  (:Triggered
    (Default|Move (Variables|Default|GetBP_MoveableComponentLAN) (.yaw (Pawn|GetControlRotation :!class /Script/Engine.Pawn)) (.x ActionValue) (.y ActionValue)))
  (:Started
    (Default|IsMoveing _bp_moveablecomponentlan true))
  (:Completed
    (Default|IsMoveing _bp_moveablecomponentlan false)))

(event Input|EnhancedActionEvents|EnhancedInputActionIA_GunnerJump
  (params (ActionValue :type Boolean) (ElapsedSeconds :type Float%20%28double-precision%29) (TriggeredSeconds :type Float%20%28double-precision%29) (InputAction :type Input%20Action%20Object%20Reference :default "/Game/Colab/LEN/GunnerIMC/IA/IA_GunnerJump.IA_GunnerJump"))
  ;[1 1 1] 시야돌리기,이동,점프
  (:Started
    (Default|JumpServer (Variables|Default|GetBP_MoveableComponentLAN))))

(event Input|EnhancedActionEvents|EnhancedInputActionIA_GunnerLook
  (params (ActionValue :type Vector%202D%20Structure) (ElapsedSeconds :type Float%20%28double-precision%29) (TriggeredSeconds :type Float%20%28double-precision%29) (InputAction :type Input%20Action%20Object%20Reference :default "/Game/Colab/LEN/GunnerIMC/IA/IA_GunnerLook.IA_GunnerLook"))
  ;[1 1 1] 시야돌리기,이동,점프
  (Pawn|Input|AddControllerYawInput (.x ActionValue))
  (Pawn|Input|AddControllerPitchInput (.y ActionValue)))

(event EventBeginPlay
  ;[1 1 1] 비긴플레이
  (bind _as플레이어_컨트롤러 (Utilities|Casting|CastToPlayerController (Pawn|GetController)))
  (Variables|Default|SetPlayerControllerRef _as플레이어_컨트롤러)
  (Utilities|IsValid (PlayerController|LocalPlayerSubsystems|GetEnhancedInputLocalPlayerSubsystem _as플레이어_컨트롤러)
    (:Is%20Valid
      (Input|AddMappingContext (PlayerController|LocalPlayerSubsystems|GetEnhancedInputLocalPlayerSubsystem _as플레이어_컨트롤러) "/Game/Colab/LEN/GunnerIMC/IMC_GunnerDefault.IMC_GunnerDefault" 0 "(bIgnoreAllPressedKeysUntilRelease=True,bForceImmediately=False,bNotifyUserSettings=False)"))))

(event EventTick
  (params (DeltaSeconds :type Float%20%28single-precision%29))
  ;[1 1 1] 틱
  (Class|PrimitiveComponent|WakeAllRigidBodies (Variables|Default|GetSkeletalMesh))
  (Networking|SwitchHasAuthority
    (:Authority
      (Default|SMoveTick (Variables|Default|GetBP_MoveableComponentLAN)))))

(fn ConstructionScript)

(fn GetHandVelocity
  (bind _bp_handmoveablecomponent (Variables|Default|GetBP_HandMoveableComponent))
  (return (Variables|/Game/Colab/LEN/Component/BP_HandMoveableComponent.BP_HandMoveableComponent_C|GetHandVelocity _bp_handmoveablecomponent) (Variables|/Game/Colab/LEN/Component/BP_HandMoveableComponent.BP_HandMoveableComponent_C|GetTargetLocation _bp_handmoveablecomponent)))