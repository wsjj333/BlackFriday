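; Test drivable kart pawn with physics-based arcade driving and Mario Kart-style drifting, using Enhanced Input.
; Each tick, four wheel line traces apply spring-like suspension forces, while smoothed throttle drives forward force, airborne downforce and center-of-mass shift.
; Steering applies throttle-scaled torque and turns the front wheels visually.
; Drifting locks steer direction, sharpens turning, yaws the body visually and grants a timed boost; driver-exit logic is unconnected.
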(event Input|EnhancedActionEvents|EnhancedInputActionIA_Acceleration
  (params (ActionValue :type Float%20%28double-precision%29) (ElapsedSeconds :type Float%20%28double-precision%29) (TriggeredSeconds :type Float%20%28double-precision%29) (InputAction :type Input%20Action%20Object%20Reference :default "/Game/Colab/CCW/Cart/Input/Actions/IA_Acceleration.IA_Acceleration"))
  ;[1 1 1] 가속 키 눌렀을 때
  (Variables|Default|SetAccelerationInput (Math|Interpolation|FInterpTo (Variables|Default|GetAccelerationInput) (Math|Float|SelectFloat ActionValue 0.0 (CallFunction|IsonGround)) (Utilities|Time|GetWorldDeltaSeconds) 0.5)))

(event Input|EnhancedActionEvents|EnhancedInputActionIA_Steer
  (params (ActionValue :type Float%20%28double-precision%29) (ElapsedSeconds :type Float%20%28double-precision%29) (TriggeredSeconds :type Float%20%28double-precision%29) (InputAction :type Input%20Action%20Object%20Reference :default "/Game/Colab/CCW/Cart/Input/Actions/IA_Steer.IA_Steer"))
  (bind _wheel_fl (Variables|Default|GetWheel_FL))
  (bind _wheel_fl_2 (Variables|Default|GetWheel_FL))
  (bind _wheel_fr (Variables|Default|GetWheel_FR))
  (bind _wheel_fr_2 (Variables|Default|GetWheel_FR))
  (bind _relativerotation (Variables|/Script/Engine.SceneComponent|GetRelativeRotation _wheel_fr_2))
  (bind _relativerotation_2 (Variables|/Script/Engine.SceneComponent|GetRelativeRotation _wheel_fr))
  (bind _relativerotation_3 (Variables|/Script/Engine.SceneComponent|GetRelativeRotation _wheel_fl))
  (bind _relativerotation_4 (Variables|/Script/Engine.SceneComponent|GetRelativeRotation _wheel_fl_2))
  ;[1 1 1] 조향
  (:Triggered
    ;;[1 1 1] 드리프트를 쉽게 멈추거나 방향을 바꿀 수 없게 하는 조작감 구현
    (bind _output_get (Variables|Default|SetDriftSteer (Math|Float|Clamp(Float) (Math|Float|SelectFloat (* (Math|Float|Max(Float) (Variables|Default|GetDriftSteer) (Math|Float|Absolute(Float) ActionValue)) (Math|Float|Sign(Float) (.yaw (Variables|Default|GetDriftRotation)))) ActionValue (Variables|Default|GetbIsDrifting)) -3.0 3.0)))
    (Class|PrimitiveComponent|AddTorqueinRadians (Variables|Default|GetBox) (Math|Vector|MakeVector 0.0 0.0 (* _output_get (Variables|Default|GetSteeringTorque) (* (Variables|Default|GetAccelerationInput) (Variables|Default|GetSteeringMultiplier)))) "None" false)
    ;;[1 1 1] 앞바퀴 조향
    (Transformation|SetRelativeRotation _wheel_fr_2 (Math|Rotator|MakeRotator (.roll _relativerotation) (.pitch _relativerotation) (Math|Interpolation|FInterpTo (.yaw _relativerotation) (* ActionValue 25.0) (Utilities|Time|GetWorldDeltaSeconds) 3.0)) false false)
    (Transformation|SetRelativeRotation _wheel_fl (Math|Rotator|MakeRotator (.roll _relativerotation_3) (.pitch _relativerotation_3) (Math|Interpolation|FInterpTo (.yaw _relativerotation_3) (* ActionValue 25.0) (Utilities|Time|GetWorldDeltaSeconds) 3.0)) false false))
  (:Completed
    ;;[1 1 1] 앞바퀴 조향을 멈추었을때 일정 시간 내에 원래 자리로 돌아가게 함
    (Timeline|Timeline PlayFromStart
      (:Update
        (Transformation|SetRelativeRotation _wheel_fl_2 (Math|Rotator|MakeRotator (.roll _relativerotation_4) (.pitch _relativerotation_4) (Math|Interpolation|FInterpTo (.yaw _relativerotation_4) 0.0 (Utilities|Time|GetWorldDeltaSeconds) 3.0)) false false)
        (Transformation|SetRelativeRotation _wheel_fr (Math|Rotator|MakeRotator (.roll _relativerotation_2) (.pitch _relativerotation_2) (Math|Interpolation|FInterpTo (.yaw _relativerotation_2) 0.0 (Utilities|Time|GetWorldDeltaSeconds) 3.0)) false false)))))

(event Input|EnhancedActionEvents|EnhancedInputActionIA_Drift
  (params (ActionValue :type Boolean) (ElapsedSeconds :type Float%20%28double-precision%29) (TriggeredSeconds :type Float%20%28double-precision%29) (InputAction :type Input%20Action%20Object%20Reference :default "/Game/Colab/CCW/Cart/Input/Actions/IA_Drift.IA_Drift"))
  ;[1 1 1] 드리프트
  (:Started
    (CallFunction|StartDrift))
  (:Canceled
    (CallFunction|StopDrift :!label _label))
  (:Completed
    (goto _label)))

(event Input|EnhancedActionEvents|EnhancedInputActionIA_Drive
  (params (ActionValue :type Boolean) (ElapsedSeconds :type Float%20%28double-precision%29) (TriggeredSeconds :type Float%20%28double-precision%29) (InputAction :type Input%20Action%20Object%20Reference :default "/Game/Colab/CCW/Characters/Input/Actions/IA_Drive.IA_Drive")))

(event EventBeginPlay
  ;[1 1 1] 초기화
  (bind _returnvalue (Actor|GetActorOfClass "/Game/Colab/CCW/Characters/Blueprints/BP_CartDriverTest.BP_CartDriverTest_C"))
  (Variables|Default|SetCartDriver _returnvalue))

(event EventPossessed
  (params (NewController :type Controller%20Object%20Reference))
  ;[1 1 1] 초기화
  (bind _as플레이어_컨트롤러 (Utilities|Casting|CastToPlayerController NewController))
  (if (Pawn|IsLocalPlayerController _as플레이어_컨트롤러)
    (Input|AddMappingContext (PlayerController|LocalPlayerSubsystems|GetEnhancedInputLocalPlayerSubsystem _as플레이어_컨트롤러) "/Game/Colab/CCW/Cart/Input/IMC_CartTest.IMC_CartTest" 0 "(bIgnoreAllPressedKeysUntilRelease=True,bForceImmediately=False,bNotifyUserSettings=False)")))

(event EventTick
  (params (DeltaSeconds :type Float%20%28single-precision%29))
  ;[1 1 1] 매 프레임 실행
  (CallFunction|SuspensionCast (Variables|Default|GetWheel_FL))
  (CallFunction|SuspensionCast (Variables|Default|GetWheel_FR))
  (CallFunction|SuspensionCast (Variables|Default|GetWheel_BL))
  (CallFunction|SuspensionCast (Variables|Default|GetWheel_BR))
  (CallFunction|AddAcceleration)
  (CallFunction|CalculateAcceleration))

(fn ConstructionScript)

(fn SuspensionCast
  (params (WheelComp :type Scene%20Component%20Object%20Reference))
  (bind _returnvalue (Transformation|GetWorldLocation WheelComp))
  (bind _returnvalue_2 (Components|GetChildComponent WheelComp 0))
  (bind _relativelocation (Variables|/Script/Engine.SceneComponent|GetRelativeLocation _returnvalue_2))
  (bind _outhit (Collision|LineTraceByChannel _returnvalue (+ _returnvalue (* (Math|Vector|GetUpVector WheelComp) -6e+01)) "TraceTypeQuery1" false 0 "ForOneFrame"))
  ;[1 1 1] 라인 트레이스로 차체 서스펜션
  (LocalVariables|SetHitResultDistance (.Distance (Collision|BreakHitResult _outhit)))
  (if (.bBlockingHit (Collision|BreakHitResult _outhit))
    (Class|PrimitiveComponent|AddForceatLocation (Variables|Default|GetBox) (* (- 1.0 (Math|Float|NormalizetoRange (.Distance (Collision|BreakHitResult _outhit)) 0.0 6e+01)) (Math|Vector|GetUnitDirection(Vector) (.TraceEnd (Collision|BreakHitResult _outhit)) (.TraceStart (Collision|BreakHitResult _outhit))) (Variables|Default|GetSuspensionForceMultiplier)) (Transformation|GetWorldLocation WheelComp) "None") ; Target(카트)의 벡터에\nLocation(Wheel Comp)를 힘의 작용점으로 해서\nForce(압축율 + 위쪽 방향) 벡터를 더한다\n즉, 서스펜션이 압축된 만큼 다시 위쪽으로 카트를 들어올린다
    ;[1 1 1] 바퀴 위치 조정
    (Transformation|SetRelativeLocation _returnvalue_2 (Math|Vector|MakeVector (.x _relativelocation) (.y _relativelocation) (Math|Interpolation|FInterpTo (.z _relativelocation) (+ (* (LocalVariables|GetHitResultDistance) -1.0) 32.0) (Utilities|Time|GetWorldDeltaSeconds) 3.0)) false false)))

(fn CalculateAcceleration
  (bind _pivot (Variables|Default|GetPivot))
  (bind _cube (Variables|Default|GetCube))
  ;[1 1 1] 비선형적인 가속 감도 구현
  (Variables|Default|SetAcceleration (* (Math|Float|Lerp 0.0 (Variables|Default|GetMaxAcceleration) (Variables|Default|GetAccelerationInput)) (Variables|Default|GetAccelerationInput) (Math|Float|Sign(Float) (Variables|Default|GetAccelerationInput))))
  ;[1 1 1] 가만히 있으면 속도 점차 줄어듦
  (Variables|Default|SetAccelerationInput (Math|Interpolation|FInterpTo (Variables|Default|GetAccelerationInput) 0.0 (Utilities|Time|GetWorldDeltaSeconds) 0.5))
  ;[1 1 1] 바퀴 회전 속도
  (Transformation|AddLocalRotation (Variables|Default|GetFLWheel) (Math|Rotator|MakeRotator 0.0 0.0 (/ (Variables|Default|GetAcceleration) -1e+03)) false false)
  ;[1 1 1] 시각적인 회전 효과 (차체, 바퀴 회전)
  (Transformation|SetRelativeRotation _pivot (Math|Interpolation|RInterpTo (Variables|/Script/Engine.SceneComponent|GetRelativeRotation _pivot) (Variables|Default|GetDriftRotation) (Utilities|Time|GetWorldDeltaSeconds) 3.0) false false)
  (Transformation|SetRelativeRotation _cube (Math|Interpolation|RInterpTo (Variables|/Script/Engine.SceneComponent|GetRelativeRotation _cube) (Variables|Default|GetDriftRotation) (Utilities|Time|GetWorldDeltaSeconds) 3.0) false false))

(fn AddAcceleration
  (bind _box (Variables|Default|GetBox))
  (Class|PrimitiveComponent|AddForceatLocation _box (+ (* (Math|Vector|GetForwardVector _box) (Variables|Default|GetAccelerationInput) (Variables|Default|GetSpeed) (Physics|GetMass _box) (Variables|Default|GetSpeedModifier)) (Math|Vector|SelectVector "0, 0, 0" (Math|Vector|MakeVector 0.0 0.0 (Variables|Default|GetDownForce)) (CallFunction|IsonGround))) (Transformation|GetWorldLocation _box) "None")
  (CallFunction|SetCartCenterOfMassLow))

(fn SetCartCenterOfMassLow
  (Class|PrimitiveComponent|SetCenterOfMass (Variables|Default|GetBox) (* "0.000000,0.000000,-10.000000" (Variables|Default|GetAccelerationInput)) "None"))

(fn IsonGround
  (bind _returnvalue (Transformation|GetActorLocation))
  (bind _returnvalue_2 (Collision|LineTraceByChannel _returnvalue (- _returnvalue (Variables|Default|GetGroundTraceEnd)) "TraceTypeQuery1" false 0 "ForOneFrame" true "(R=0.082094,G=0.000000,B=1.000000,A=1.000000)" "(R=1.000000,G=0.037092,B=0.979415,A=1.000000)"))
  (return _returnvalue_2))

(fn BoostCart
  (params (SpeedModifier :type Float%20%28single-precision%29) (Time :type Float%20%28single-precision%29))
  (Variables|Default|SetSpeedModifier SpeedModifier)
  (Utilities|Time|SetTimerbyFunctionName 0 "ResetSpeed" Time))

(fn ResetSpeed
  (Variables|Default|SetSpeedModifier 1.0))

(fn StartDrift
  (Variables|Default|SetSteeringMultiplier 4.0)
  (Variables|Default|SetbIsDrifting true)
  (Variables|Default|SetDriftRotation (Math|Rotator|MakeRotator 0.0 0.0 (* (Math|Float|Sign(Float) (Input|EnhancedActionValues|GetIA_Steer)) 25.0)))
  ;[1 1 1] 마리오 카트처럼 드리프트할 때 속도 올려주는 기능
  (CallFunction|BoostCart (+ (/ (Math|Float|Absolute(Float) (Variables|Default|GetDriftSteer)) 1e+01) 1.0) 1.0))

(fn StopDrift
  (Variables|Default|SetSteeringMultiplier 2.0)
  (Variables|Default|SetbIsDrifting false)
  (Variables|Default|SetDriftRotation "0, 0, 0"))