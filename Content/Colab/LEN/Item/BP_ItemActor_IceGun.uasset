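; BP_ItemActor_IceGun is an ice gun item actor whose GunFire function shoots pre-existing bullets from a pool.
; Each shot decrements GunBullets, instantly refilling to ten when empty, and prints debug messages.
; The bullet at GunBullets - 1 after decrementing, if valid, launches via FireNormal from GunSocket's location and rotation.
; TargetLocation, IsHit and the computed forward target go unused, and the event graph holds only inactive stubs.
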(event EventBeginPlay
  (|CallParentFunction) ; 지금 이 노드는 비활성 상태입니다. \n핀을 끌어서 다른 노드를 연결하면 활성화됩니다.
)

(event Collision|EventActorBeginOverlap
  (params (OtherActor :type Actor%20Object%20Reference)))

(event EventTick
  (params (DeltaSeconds :type Float%20%28single-precision%29))
  (|CallParentFunction DeltaSeconds) ; 지금 이 노드는 비활성 상태입니다. \n핀을 끌어서 다른 노드를 연결하면 활성화됩니다.
)

(fn ConstructionScript
  (|CallParentFunction))

(fn GunFire
  (params (TargetLocation :type Vector :default "0, 0, 0") (IsHit :type Boolean))
  (bind _staticmesh (Variables|Default|GetStaticMesh))
  (bind _staticmesh_2 (Variables|Default|GetStaticMesh))
  (if (> (Variables|Default|GetGunBullets) 0)
    _
    (else
      (Development|PrintString "재장전")
      (Variables|Default|SetGunBullets 10)))
  (Development|PrintString "발사")
  (Math|Integer|DecrementInt (Variables|Default|GetGunBullets)
    (:%20%20
      (if (Utilities|IsValid (Utilities|Array|Get(acopy) (Variables|Default|GetBullets) (- (Variables|Default|GetGunBullets) 1)))
        (LocalVariables|SetNewTarget (+ (Transformation|GetSocketLocation _staticmesh "GunSocket") (* (Math|Vector|GetForwardVector (Transformation|GetSocketRotation _staticmesh "GunSocket")) 1e+03)))
        ;[1 1 1] 총알 활성화
        (Default|FireNormal (Utilities|Array|Get(acopy) (Variables|Default|GetBullets) (- (Variables|Default|GetGunBullets) 1)) (Transformation|GetSocketLocation _staticmesh_2 "GunSocket") (Transformation|GetSocketRotation _staticmesh_2 "GunSocket"))))))