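; Actor component that lets a pawn be blinded by an item effect, shown as a screen overlay for the local player.
; BeginPlay caches the owning pawn, and ItemEffectBlindStart runs only if it is locally controlled and not already blind.
; It creates a WBP_BlindEffect widget, binds an event to its timer end, starts the effect and adds it to the viewport.
; ItemEffectBlindEnd clears the blind flag and widget reference.
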(event EventBeginPlay
  (bind _as폰 (Utilities|Casting|CastToPawn (Components|GetOwner)))
  (Variables|Default|SetOwnerPawn _as폰))

(fn ItemEffectBlindStart
  (bind _ownerpawn (Variables|Default|GetOwnerPawn)
    (:then
      (if (Pawn|IsLocallyControlled _ownerpawn)
        (if (not (Variables|Default|GetbIsBlind))
          (Variables|Default|SetbIsBlind true)
          (bind _returnvalue (UserInterface|CreateWidget "/Game/Colab/LEN/WB/WBP_BlindEffect.WBP_BlindEffect_C"))
          (Variables|Default|SetBlindEffectWidget _returnvalue)
          (EventDispatchers|BindEventtoTimerEnd (Variables|Default|GetBlindEffectWidget) (EventDispatchers|CreateEvent :!event ItemEffectBlindEnd))
          (Default|StartBlindEffect (Variables|Default|GetBlindEffectWidget))
          (UserInterface|Viewport|AddtoViewport (Variables|Default|GetBlindEffectWidget) 0))))
    (:else)))

(fn ItemEffectBlindEnd
  (Variables|Default|SetbIsBlind false)
  (Variables|Default|SetBlindEffectWidget 0)
  (Development|PrintString "블라인드 해제"))