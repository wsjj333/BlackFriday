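; Base gun item actor that fires hitscan shots and switches the holder's gun state on attach and detach.
; On BeginPlay it pre-spawns a pool of BP_Bullet actors, one per round, each linked back to the gun.
; Attach and detach call ActiveGun and NotActiveGun on the owner's BP_ItemPickableCharacter component.
; GunFire auto-refills an empty magazine, decrements the count and fires a pooled bullet from GunSocket toward the target.
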(event EventAttachHand
  (params (Actor :type Actor%20Object%20Reference))
  (bind _itemowner (Variables|Default|GetItemOwner))
  (bind _returnvalue (Actor|GetComponentbyClass _itemowner "/Game/Colab/LEN/Component/BP_ItemPickableCharacter.BP_ItemPickableCharacter_C"))
  (|CallParentFunction Actor)
  (if (Utilities|Enum|Equal(Enum) (Variables|Default|GetAttackType) "NewEnumerator5")
    (bind _output_get (Variables|Default|SetItemComponent _returnvalue))
    (Default|ActiveGun _returnvalue)))

(event EventDettachHand
  (|CallParentFunction)
  (if (Utilities|Enum|Equal(Enum) (Variables|Default|GetAttackType) "NewEnumerator5")
    (bind _itemcomponent (Variables|Default|GetItemComponent)
      (:then
        (Default|NotActiveGun _itemcomponent)
        (Variables|Default|SetItemComponent 0))
      (:else))))

(event EventBeginPlay
  (|CallParentFunction)
  (Variables|Default|SetAttackType "NewEnumerator5")
  (CallFunction|SpawnBullet))

(fn ConstructionScript
  (|CallParentFunction))

(fn GunFire
  (params (TargetLocation :type Vector) (IsHit :type Boolean))
  (if (> (Variables|Default|GetGunBullets) 0)
    _
    (else
      (Development|PrintString "재장전")
      (Variables|Default|SetGunBullets 10)))
  (Development|PrintString "발사")
  (Math|Integer|DecrementInt (Variables|Default|GetGunBullets)
    (:%20%20
      (if (Utilities|IsValid (Utilities|Array|Get(acopy) (Variables|Default|GetBullets) (- (Variables|Default|GetGunBullets) 1)))
        ;[1 1 1] 총알 활성화
        (Default|FireHitScan (Utilities|Array|Get(acopy) (Variables|Default|GetBullets) (- (Variables|Default|GetGunBullets) 1)) (Transformation|GetSocketLocation (Variables|Default|GetStaticMesh) "GunSocket") TargetLocation IsHit)))))

(fn SpawnBullet
  (for _index (range 1 (Variables|Default|GetGunBullets))
    (bind _returnvalue (Game|SpawnActorfromClass "/Game/Colab/LEN/Item/BP_Bullet.BP_Bullet_C" (Math|Transform|MakeTransform "0, 0, 0" "0, 0, 0" "1.000000,1.000000,1.000000") "Undefined" "MultiplyWithRoot" 0 self 0))
    (Utilities|Array|Add (Variables|Default|GetBullets) _returnvalue)))