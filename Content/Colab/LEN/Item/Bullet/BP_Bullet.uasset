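; BP_Bullet is a reusable gun bullet that hides and deactivates instead of being destroyed.
; FireNormal launches it via ProjectileMovement, ignoring the gun and its owner, until timeout or capsule hit, which explodes and pushes targets with BP_HitableComponent.
; FireHitScan disables collision and moves a purely visual bullet to a supplied target, spawning any impact effect immediately at launch.
; BulletState selects Tick and deactivation behavior for each mode.
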(event OnComponentHit(Capsule)
  (params (HitComponent :type Primitive%20Component%20Object%20Reference) (OtherActor :type Actor%20Object%20Reference) (OtherComp :type Primitive%20Component%20Object%20Reference) (NormalImpulse :type Vector :default "0, 0, 0") (Hit :type Hit%20Result%20Structure%20%28by%20ref%29))
  (bind _returnvalue (Actor|GetComponentbyClass OtherActor "/Game/Colab/LEN/Component/ItemComponents/BP_HitableComponent.BP_HitableComponent_C"))
  (CallFunction|BulletExplosionEffect (.ImpactPoint (Collision|BreakHitResult Hit)))
  (CallFunction|BulletDeactivate)
  (Utilities|IsValid _returnvalue
    (:Is%20Valid
      (Default|AddAttackForce _returnvalue 0.0 (* (Transformation|GetActorForwardVector) 5e+02) "None" true true))))

(event EventBeginPlay
  ;[1 1 1] 발사중인 총은 충돌되지 않게
  (bind _owninggun (Variables|Default|GetOwningGun)
    (:then
      (Collision|IgnoreActorwhenMoving (Variables|Default|GetCapsule) _owninggun true))
    (:else)))

(event EventTick
  (params (DeltaSeconds :type Float%20%28single-precision%29))
  (switch Utilities|FlowControl|Switch|SwitchonE_BulletState (Variables|Default|GetBulletState)
    (:NewEnumerator1
      (CallFunction|NormalFireTick DeltaSeconds))
    (:NewEnumerator2
      (CallFunction|HitScanFireTick DeltaSeconds))))

(fn ConstructionScript)

(fn FireHitScan
  (params (BulletStartLocation :type Vector) (TargetLocation :type Vector) (IsHit :type Boolean))
  (bind _capsule (Variables|Default|GetCapsule))
  (Variables|Default|SetTargetLocation TargetLocation)
  (bind _returnvalue (Transformation|SetActorLocation BulletStartLocation false false))
  (if _returnvalue
    (Variables|Default|SetBulletState "NewEnumerator2")
    (if (Class|PrimitiveComponent|IsCollisionEnabled _capsule)
      (Collision|SetCollisionEnabled _capsule "NoCollision"))
    (Actor|Tick|SetActorTickEnabled true)
    (Development|SetHiddeninGame (Variables|Default|GetCube) false false)
    (if IsHit
      (CallFunction|BulletExplosionEffect (Variables|Default|GetTargetLocation)))))

(fn FireNormal
  (params (BulletStartLocation :type Vector) (BulletStartRotaion :type Rotator))
  (bind _returnvalue (Transformation|SetActorLocationAndRotation BulletStartLocation BulletStartRotaion))
  (if _returnvalue
    (Variables|Default|SetBulletState "NewEnumerator1")
    (Collision|SetCollisionEnabled (Variables|Default|GetCapsule) "QueryOnly")
    (CallFunction|SetIgnoreActor)
    (Development|SetHiddeninGame (Variables|Default|GetCube) false false)
    (Game|Components|ProjectileMovement|SetVelocityinLocalSpace (Variables|Default|GetProjectileMovement) "3000.000000,0.000000,0.000000")
    (Components|Activation|SetActive (Variables|Default|GetProjectileMovement) true true)
    (Variables|Default|SetNormalFireAccTime 0.0)))

(fn HitScanFireTick
  (params (DeltaTime :type Float%20%28single-precision%29))
  (Transformation|SetActorLocationAndRotation (Math|Interpolation|VInterptoConstant (Transformation|GetActorLocation) (Variables|Default|GetTargetLocation) DeltaTime (Variables|Default|GetBulletSpeed)) (Math|Rotator|FindLookatRotation (Transformation|GetActorLocation) (Variables|Default|GetTargetLocation)))
  (if (Utilities|Operators|EqualEqual (Transformation|GetActorLocation) (Variables|Default|GetTargetLocation) 1.0)
    (CallFunction|BulletDeactivate)))

(fn NormalFireTick
  (params (DeltaTime :type Float%20%28single-precision%29))
  (bind _output_get (Variables|Default|SetNormalFireAccTime (+ (Variables|Default|GetNormalFireAccTime) DeltaTime)))
  (if (>= _output_get (Variables|Default|GetNormalFireDelayTime))
    (CallFunction|BulletDeactivate)))

(fn BulletDeactivate
  (switch Utilities|FlowControl|Switch|SwitchonE_BulletState (Variables|Default|GetBulletState)
    (:NewEnumerator1
      (Variables|Default|SetBulletState "NewEnumerator0")
      (Collision|SetCollisionEnabled (Variables|Default|GetCapsule) "NoCollision")
      (Development|SetHiddeninGame (Variables|Default|GetCube) true false)
      (Components|Activation|SetActive (Variables|Default|GetProjectileMovement) false true)
      (CallFunction|RemoveIgnoreActor))
    (:NewEnumerator2
      (Variables|Default|SetBulletState "NewEnumerator0")
      (Collision|SetCollisionEnabled (Variables|Default|GetCapsule) "NoCollision")
      (Development|SetHiddeninGame (Variables|Default|GetCube) true false)
      (Actor|Tick|SetActorTickEnabled false))))

(fn BulletExplosionEffect
  (params (Location :type Vector))
  (Effects|SpawnEmitteratLocation (Variables|Default|GetExplosionPaticle) Location "0, 0, 0" "0.500000,0.500000,0.500000")
  (Development|PrintString "맞았다"))

(fn SetIgnoreActor
  (Utilities|IsValid (Variables|Default|GetIgnoreActor)
    (:Is%20Not%20Valid
      (bind _itemowner (Variables|/Game/Colab/LEN/Item/BP_ItemActor.BP_ItemActor_C|GetItemOwner (Variables|Default|GetOwningGun))
        (:then
          (bind _output_get (Variables|Default|SetIgnoreActor _itemowner))
          (Collision|IgnoreActorwhenMoving (Variables|Default|GetCapsule) _output_get true))
        (:else)))))

(fn RemoveIgnoreActor
  (bind _ignoreactor (Variables|Default|GetIgnoreActor)
    (:then
      (Collision|IgnoreActorwhenMoving (Variables|Default|GetCapsule) _ignoreactor false)
      (Variables|Default|SetIgnoreActor 0))
    (:else)))