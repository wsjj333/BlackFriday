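; BP_Bullet is a reusable bullet actor that flies a visible cube from a start point to a fixed target location.
; BulletFireStart stores the target, teleports or moves the actor to the start, and on success shows the cube and enables flight.
; Tick moves it at constant speed facing the target, then on arrival hides the cube, stops flight and prints a hit message.
; Hits are purely distance-based, with no damage applied.
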(event EventTick
  (params (DeltaSeconds :type Float%20%28single-precision%29))
  (if (Variables|Default|GetbIsFire)
    (Transformation|SetActorLocationAndRotation (Math|Interpolation|VInterptoConstant (Transformation|GetActorLocation) (Variables|Default|GetTargetLocation) DeltaSeconds (Variables|Default|GetBulletSpeed)) (Math|Rotator|FindLookatRotation (Transformation|GetActorLocation) (Variables|Default|GetTargetLocation)))
    (if (Utilities|Operators|EqualEqual (Transformation|GetActorLocation) (Variables|Default|GetTargetLocation) 1.0)
      (Variables|Default|SetbIsFire false)
      (Development|SetHiddeninGame (Variables|Default|GetCube) true false)
      (Development|PrintString "맞았다"))))

(fn ConstructionScript)

(fn BulletFireStart
  (params (BulletStartLocation :type Vector) (TargetLocation :type Vector))
  (Variables|Default|SetTargetLocation TargetLocation)
  (bind _returnvalue (Transformation|SetActorLocation BulletStartLocation false false))
  (if _returnvalue
    (Variables|Default|SetbIsFire true)
    (Development|SetHiddeninGame (Variables|Default|GetCube) false false)))