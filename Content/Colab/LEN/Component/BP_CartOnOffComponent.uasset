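; Pawn component that lets a gunner board and leave a tagged cart, initialized through the IsBeginPlay RepNotify.
; Input relays through S_/SC_ events to a sphere trace that attaches the pawn to the cart's riding point, or detaches it.
; Riding swaps input contexts, disables physics and ticks local yaw from control rotation.
; Collision goes Ignore while riding, Overlap on dismount, then Block after leaving the cart's overlap.
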(event Custom|S_RidingOnOff
  (CallFunction|SCRidingonOff))

(event Custom|EndOverlap
  (params (OverlappedComponent :type Primitive%20Component%20Object%20Reference) (OtherActor :type Actor%20Object%20Reference) (OtherComp :type Primitive%20Component%20Object%20Reference) (OtherBodyIndex :type Integer))
  (if (not (Variables|Default|GetbIsRiding))
    (if (Actor|ActorHasTag OtherActor (Variables|Default|GetTagNameActor))
      (Development|PrintString "카트범위 벗어남")
      (Collision|SetCollisionResponsetoChannel (Variables|Default|GetOwnersRoot) "ECC_GameTraceChannel2" "ECR_Block"))))

(event Custom|TickMouseLook
  (params (NewRotation :type Rotator))
  (Transformation|SetActorRotation (Variables|Default|GetPawnOwner) NewRotation))

(event Custom|SC_RidingOnOff
  (if (Variables|Default|GetbIsRiding)
    (CallFunction|UnRiding)
    (else
      (CallFunction|TryRiding))))

(event Custom|CustomBeginPlay
  (Components|Tick|SetComponentTickEnabled false)
  ;[1 1 1] 오너 가져오기
  (bind _as폰 (Utilities|Casting|CastToPawn (Components|GetOwner)))
  (bind _output_get (Variables|Default|SetPawnOwner _as폰))
  ;[1 1 1] 오너의 스켈레탈 가져오기
  (Variables|Default|SetOwnersSkeletal (Actor|GetComponentbyClass _output_get "/Script/Engine.SkeletalMeshComponent"))
  ;[1 1 1] 매핑 컨텍스트
  (bind _as플레이어_컨트롤러 (Utilities|Casting|CastToPlayerController (Pawn|GetController (Variables|Default|GetPawnOwner)))
    (:then
      (Variables|Default|SetOwnerPlayerController _as플레이어_컨트롤러)
      (Utilities|IsValid (PlayerController|LocalPlayerSubsystems|GetEnhancedInputLocalPlayerSubsystem _as플레이어_컨트롤러)
        (:Is%20Valid
          (Input|AddMappingContext (PlayerController|LocalPlayerSubsystems|GetEnhancedInputLocalPlayerSubsystem _as플레이어_컨트롤러) "/Game/Colab/LEN/GunnerIMC/IMC_CartRidingOnOff.IMC_CartRidingOnOff" 0 "(bIgnoreAllPressedKeysUntilRelease=True,bForceImmediately=False,bNotifyUserSettings=False)"))))
    (:CastFailed
      _))
  (bind _as프리미티브_컴포넌트 (Utilities|Casting|CastToPrimitiveComponent (Variables|/Script/Engine.Actor|GetRootComponent (Variables|Default|GetPawnOwner))))
  (bind _output_get_2 (Variables|Default|SetOwnersRoot _as프리미티브_컴포넌트))
  (Collision|BindEventtoOnComponentEndOverlap _output_get_2 (delegate Custom|EndOverlap)))

(event Input|EnhancedActionEvents|EnhancedInputActionIA_CartRidingOnOff
  (params (ActionValue :type Boolean) (ElapsedSeconds :type Float%20%28double-precision%29) (TriggeredSeconds :type Float%20%28double-precision%29) (InputAction :type Input%20Action%20Object%20Reference :default "/Game/Colab/LEN/GunnerIMC/IA/IA_CartRidingOnOff.IA_CartRidingOnOff"))
  (:Started
    (CallFunction|SRidingonOff)))

(event Input|EnhancedActionEvents|EnhancedInputActionIA_GunnerLook
  (params (ActionValue :type Vector%202D%20Structure) (ElapsedSeconds :type Float%20%28double-precision%29) (TriggeredSeconds :type Float%20%28double-precision%29) (InputAction :type Input%20Action%20Object%20Reference :default "/Game/Colab/LEN/GunnerIMC/IA/IA_GunnerLook.IA_GunnerLook"))
  (bind _pawnowner (Variables|Default|GetPawnOwner))
  (if (Variables|Default|GetbIsRiding)
    (Pawn|Input|AddControllerYawInput _pawnowner (.x ActionValue))
    (Pawn|Input|AddControllerPitchInput _pawnowner (.y ActionValue))))

(event EventBeginPlay
  (Variables|Default|SetbIsBeginPlay true))

(event EventTick
  (params (DeltaSeconds :type Float%20%28single-precision%29))
  (CallFunction|LookTick))

(fn UnRiding
  (Variables|Default|SetbIsRiding false)
  (Variables|Default|SetRidingPoint 0)
  (bind _ownerplayercontroller (Variables|Default|GetOwnerPlayerController)
    (:then
      (Input|RemoveMappingContext (PlayerController|LocalPlayerSubsystems|GetEnhancedInputLocalPlayerSubsystem _ownerplayercontroller) "/Game/Colab/LEN/GunnerIMC/IMC_GunnerRiding.IMC_GunnerRiding" "(bIgnoreAllPressedKeysUntilRelease=True,bForceImmediately=False,bNotifyUserSettings=False)")
      (Input|AddMappingContext (PlayerController|LocalPlayerSubsystems|GetEnhancedInputLocalPlayerSubsystem _ownerplayercontroller) "/Game/Colab/LEN/GunnerIMC/IMC_GunnerDefault.IMC_GunnerDefault" 0 "(bIgnoreAllPressedKeysUntilRelease=True,bForceImmediately=False,bNotifyUserSettings=False)"))
    (:else
      _))
  (Transformation|DetachFromActor (Variables|Default|GetPawnOwner) "KeepWorld" "KeepWorld" "KeepWorld")
  (Physics|SetSimulatePhysics (Variables|Default|GetOwnersRoot) true)
  (Collision|SetCollisionResponsetoChannel (Variables|Default|GetOwnersRoot) "ECC_GameTraceChannel2" "ECR_Overlap")
  (Components|Tick|SetComponentTickEnabled false))

(fn TryRiding
  (bind _pawnowner (Variables|Default|GetPawnOwner))
  (bind _returnvalue (Transformation|GetActorLocation _pawnowner))
  (bind (_outhit _returnvalue_2) (Collision|SphereTraceForObjects _returnvalue _returnvalue 1.5e+02 (Utilities|Array|MakeArray "ObjectTypeQuery7") false 0 "None"))
  (if _returnvalue_2
    (if (Actor|ActorHasTag (.HitActor (Collision|BreakHitResult _outhit)) (Variables|Default|GetTagNameActor))
      (Utilities|IsValid (Class|Actor|FindComponentbyTag (.HitActor (Collision|BreakHitResult _outhit)) "/Script/Engine.SceneComponent" (Variables|Default|GetTagNameRidingPoint))
        (:Is%20Valid
          (Variables|Default|SetRidingPoint (Class|Actor|FindComponentbyTag (.HitActor (Collision|BreakHitResult _outhit)) "/Script/Engine.SceneComponent" (Variables|Default|GetTagNameRidingPoint)))
          (Development|PrintString "탑승")
          (bind _ownerplayercontroller (Variables|Default|GetOwnerPlayerController)
            (:then
              (Input|RemoveMappingContext (PlayerController|LocalPlayerSubsystems|GetEnhancedInputLocalPlayerSubsystem _ownerplayercontroller) "/Game/Colab/LEN/GunnerIMC/IMC_GunnerDefault.IMC_GunnerDefault" "(bIgnoreAllPressedKeysUntilRelease=True,bForceImmediately=False,bNotifyUserSettings=False)")
              (Input|AddMappingContext (PlayerController|LocalPlayerSubsystems|GetEnhancedInputLocalPlayerSubsystem _ownerplayercontroller) "/Game/Colab/LEN/GunnerIMC/IMC_GunnerRiding.IMC_GunnerRiding" 0 "(bIgnoreAllPressedKeysUntilRelease=True,bForceImmediately=False,bNotifyUserSettings=False)"))
            (:else
              _))
          (CallFunction|CartAttach)
          (Components|Tick|SetComponentTickEnabled true))))))

(fn LookTick
  (if (Variables|Default|GetbIsRiding)
    (bind _pawnowner (Variables|Default|GetPawnOwner)
      (:then
        (if (Pawn|IsLocallyControlled _pawnowner)
          (CallFunction|TickMouseLook (Math|Rotator|MakeRotator 0.0 0.0 (.yaw (Pawn|GetControlRotation (Variables|Default|GetPawnOwner) :!class /Script/Engine.Pawn)))) ; 마우스 움직임에 따라 로테이트
        ))
      (:else))))

(fn CartAttach
  (if (and (Utilities|IsValid (Variables|Default|GetOwnersRoot)) (Utilities|IsValid (Variables|Default|GetOwnersRoot)))
    (Physics|SetPhysicsLinearVelocity (Variables|Default|GetOwnersRoot) "0, 0, 0" false "None")
    (Collision|SetCollisionResponsetoChannel (Variables|Default|GetOwnersRoot) "ECC_GameTraceChannel2" "ECR_Ignore")
    (Physics|SetSimulatePhysics (Variables|Default|GetOwnersRoot) false)
    (Transformation|SetActorLocation (Variables|Default|GetPawnOwner) (Transformation|GetWorldLocation (Variables|Default|GetRidingPoint)) false false)
    (Transformation|AttachComponentToComponent (Variables|Default|GetPawnOwner) (Variables|Default|GetRidingPoint) "None" "SnapToTarget" "SnapToTarget" "KeepWorld" true)
    (Variables|Default|SetbIsRiding true)))

(fn OnRepBIsBeginPlay
  (CallFunction|CustomBeginPlay))