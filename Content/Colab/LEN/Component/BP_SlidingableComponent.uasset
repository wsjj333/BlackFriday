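; Component that applies an item-triggered slip effect to a Pawn with a physics-simulated root component.
; On start, it clears a Movable flag, removes angular damping, adds a yaw spin, pushes the pawn along its velocity and starts a looping timer.
; The sliding tick function counts down about a second, then restores high angular damping, re-enables Movable and clears the timer.
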(event EventBeginPlay
  (bind _returnvalue (Components|GetOwner))
  (bind _as폰 (Utilities|Casting|CastToPawn _returnvalue))
  (Variables|Default|SetOwnerPawn _as폰)
  (bind _as프리미티브_컴포넌트 (Utilities|Casting|CastToPrimitiveComponent (Variables|/Script/Engine.Actor|GetRootComponent _returnvalue)))
  (if (Physics|IsSimulatingPhysics _as프리미티브_컴포넌트 "None")
    (Variables|Default|SetPawnsPhysicsRoot _as프리미티브_컴포넌트)))

(fn ItemEffectSlidingStart
  (bind _pawnsphysicsroot (Variables|Default|GetPawnsPhysicsRoot))
  (if (and (Utilities|IsValid (Variables|Default|GetPawnsPhysicsRoot)) (Utilities|IsValid (Variables|Default|GetOwnerPawn)))
    (Development|PrintString "미끄덩")
    (if (not (Variables|Default|GetbIsSlinding))
      (Variables|Default|SetbIsSlinding true)
      (Variables|Default|SetbMovable false)
      (Class|PrimitiveComponent|SetAngularDamping _pawnsphysicsroot 0.0)
      (Class|PrimitiveComponent|AddAngularImpulseinDegrees _pawnsphysicsroot (Math|Vector|MakeVector 0.0 0.0 7e+02) "None" true)
      (Physics|AddImpulse (Variables|Default|GetPawnsPhysicsRoot) (* (Math|Vector|Normalize (Transformation|GetVelocity (Variables|Default|GetOwnerPawn))) 5e+02) "None" true)
      (Variables|Default|SetSlindingTime 1.0)
      (bind _returnvalue (Utilities|Time|SetTimerbyEvent (EventDispatchers|CreateEvent :!event ItemEffectSlidingTick) 0.1 true))
      (Variables|Default|SetSlindingHandle _returnvalue))))

(fn ItemEffectSlidingTick
  (Variables|Default|SetSlindingTime (- (Variables|Default|GetSlindingTime) 0.1))
  (if (<= (Variables|Default|GetSlindingTime) 0.0)
    (Class|PrimitiveComponent|SetAngularDamping (Variables|Default|GetPawnsPhysicsRoot) 1e+02)
    (Variables|Default|SetbIsSlinding false)
    (Variables|Default|SetbMovable true)
    (Utilities|Time|ClearandInvalidateTimerbyHandle (Variables|Default|GetSlindingHandle))))