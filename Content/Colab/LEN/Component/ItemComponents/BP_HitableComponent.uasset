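; Component that applies attack impulses to a physics-simulating owner Pawn, on its skeletal mesh bones, its root or both.
; BeginPlay sets a RepNotify flag whose OnRep caches the simulating root primitive and, only if that succeeds, the simulating skeletal mesh.
; AddAttackForce applies velocity-change impulses to the named bone and root as selected by its flags.
; Its DamageAmount input is unused.
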(event Custom|CustomBeginPlay
  (bind _as폰 (Utilities|Casting|CastToPawn (Components|GetOwner)))
  (bind _as프리미티브_컴포넌트 (Utilities|Casting|CastToPrimitiveComponent (Variables|/Script/Engine.Actor|GetRootComponent _as폰)))
  (if (Class|SceneComponent|IsAnySimulatingPhysics _as프리미티브_컴포넌트)
    (Variables|Default|SetPhysicsRoot _as프리미티브_컴포넌트)
    (if (Class|SceneComponent|IsAnySimulatingPhysics (Actor|GetComponentbyClass _as폰 "/Script/Engine.SkeletalMeshComponent"))
      (Variables|Default|SetOwnersSkeletal (Actor|GetComponentbyClass _as폰 "/Script/Engine.SkeletalMeshComponent")))))

(event EventBeginPlay
  (Variables|Default|SetbIsBegin true))

(fn AddAttackForce
  (params (DamageAmount :type Float%20%28double-precision%29) (ImpulseAmount :type Vector) (ImpulseBoneName :type Name) (Skeletal :type Boolean) (Root :type Boolean))
  (Utilities|FlowControl|Sequence
    (:then_0
      (if Skeletal
        (bind _ownersskeletal (Variables|Default|GetOwnersSkeletal)
          (:then
            (if (Physics|IsSimulatingPhysics _ownersskeletal ImpulseBoneName)
              (Physics|AddImpulse _ownersskeletal ImpulseAmount ImpulseBoneName true)))
          (:else))))
    (:then_1
      (if Root
        (bind _physicsroot (Variables|Default|GetPhysicsRoot)
          (:then
            (Physics|AddImpulse _physicsroot ImpulseAmount "None" true))
          (:else))))))

(fn OnRepBIsBegin
  (CallFunction|CustomBeginPlay))