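; Actor component for a slip item effect that sends a physics-simulated pawn spinning and sliding without control.
; BeginPlay caches the pawn, its simulating root primitive and player controller.
; ItemEffectSlidingStart removes the gunner input mapping, zeroes angular damping, adds yaw spin and a velocity-aligned impulse, then starts a looping timer.
; ItemEffectSlidingTick counts down about a second, then sets high angular damping, adds MoveMappingContext and clears the timer.
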(event EventBeginPlay
  (bind _returnvalue (Components|GetOwner))
  (bind _as폰 (Utilities|Casting|CastToPawn _returnvalue))
  (Variables|Default|SetOwnerPawn _as폰)
  (bind _as프리미티브_컴포넌트 (Utilities|Casting|CastToPrimitiveComponent (Variables|/Script/Engine.Actor|GetRootComponent _returnvalue)))
  (if (Class|SceneComponent|IsAnySimulatingPhysics _as프리미티브_컴포넌트)
    (Variables|Default|SetPawnsPhysicsRoot _as프리미티브_컴포넌트)
    (bind _as플레이어_컨트롤러 (Utilities|Casting|CastToPlayerController (Pawn|GetController (Variables|Default|GetOwnerPawn))))
    (Variables|Default|SetOwnerPlayerController _as플레이어_컨트롤러)))

(fn ItemEffectSlidingStart
  (bind _ownerplayercontroller (Variables|Default|GetOwnerPlayerController))
  (if (and (Utilities|IsValid (Variables|Default|GetPawnsPhysicsRoot)) (Utilities|IsValid (Variables|Default|GetOwnerPawn)))
    (Development|PrintString "미끄덩")
    (if (not (Variables|Default|GetbIsSlinding))
      (Variables|Default|SetbIsSlinding true)
      (Utilities|IsValid _ownerplayercontroller
        (:Is%20Valid
          (Input|RemoveMappingContext (PlayerController|LocalPlayerSubsystems|GetEnhancedInputLocalPlayerSubsystem _ownerplayercontroller) "/Game/Colab/LEN/GunnerIMC/IMC_GunnerDefault.IMC_GunnerDefault" "(bIgnoreAllPressedKeysUntilRelease=True,bForceImmediately=False,bNotifyUserSettings=False)"))
        (:Is%20Not%20Valid
          _))
      (Class|PrimitiveComponent|SetAngularDamping (Variables|Default|GetPawnsPhysicsRoot) 0.0)
      (Class|PrimitiveComponent|AddAngularImpulseinDegrees (Variables|Default|GetPawnsPhysicsRoot) (Math|Vector|MakeVector 0.0 0.0 7e+02) "None" true)
      (Physics|AddImpulse (Variables|Default|GetPawnsPhysicsRoot) (* (Math|Vector|Normalize (Transformation|GetVelocity (Variables|Default|GetOwnerPawn))) 5e+02) "None" true)
      (Variables|Default|SetSlindingTime 1.0)
      (bind _returnvalue (Utilities|Time|SetTimerbyEvent (EventDispatchers|CreateEvent :!event ItemEffectSlidingTick) 0.1 true))
      (Variables|Default|SetSlindingHandle _returnvalue))))

(fn ItemEffectSlidingTick
  (Variables|Default|SetSlindingTime (- (Variables|Default|GetSlindingTime) 0.1))
  (if (<= (Variables|Default|GetSlindingTime) 0.0)
    (Class|PrimitiveComponent|SetAngularDamping (Variables|Default|GetPawnsPhysicsRoot) 1e+02)
    (Variables|Default|SetbIsSlinding false)
    (bind _ownerplayercontroller (Variables|Default|GetOwnerPlayerController)
      (:then
        (Input|AddMappingContext (PlayerController|LocalPlayerSubsystems|GetEnhancedInputLocalPlayerSubsystem _ownerplayercontroller) (Variables|Default|GetMoveMappingContext) 0 "(bIgnoreAllPressedKeysUntilRelease=True,bForceImmediately=False,bNotifyUserSettings=False)"))
      (:else
        _))
    (Utilities|Time|ClearandInvalidateTimerbyHandle (Variables|Default|GetSlindingHandle))))