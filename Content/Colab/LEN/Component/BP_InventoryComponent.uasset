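; Inventory component that collects item actors released inside its owner's inventory volume, which the handlers treat as a cart.
; On BeginPlay it finds the owner's shape component tagged "Inventory" and binds overlap begin and end events.
; Overlaps notify each BP_ItemActor; entry also binds its hand-detach event, whose handler adds the item uniquely to Items and unbinds.
; Leaving the volume does not remove that binding.
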(event Custom|CartCollisionOverlapStart
  (params (OverlappedComponent :type Primitive%20Component%20Object%20Reference) (OtherActor :type Actor%20Object%20Reference) (OtherComp :type Primitive%20Component%20Object%20Reference) (OtherBodyIndex :type Integer) (bFromSweep :type Boolean) (SweepResult :type Hit%20Result%20Structure%20%28by%20ref%29))
  (bind _asbp_item_actor (Utilities|Casting|CastToBP_ItemActor OtherActor))
  (Default|OverlapCartCollision _asbp_item_actor)
  (EventDispatchers|BindEventtoOnDettachHand _asbp_item_actor (delegate Custom|DettachedItemPickUP)))

(event Custom|DettachedItemPickUP
  (params (Item :type BP%20Item%20Actor%20Object%20Reference))
  (Utilities|Array|AddUnique (Variables|Default|GetItems) Item)
  (EventDispatchers|UnbindallEventsfromOnDettachHand Item)
  (Development|PrintString "적재"))

(event Custom|CartCollisionOverlapEnd
  (params (OverlappedComponent :type Primitive%20Component%20Object%20Reference) (OtherActor :type Actor%20Object%20Reference) (OtherComp :type Primitive%20Component%20Object%20Reference) (OtherBodyIndex :type Integer))
  (bind _asbp_item_actor (Utilities|Casting|CastToBP_ItemActor OtherActor))
  (Default|UnOverlapCartCollision _asbp_item_actor))

(event EventBeginPlay
  (bind _output_get (Variables|Default|SetNewVar (Components|GetOwner)))
  (Variables|Default|SetOwnersInvenCollision (Class|Actor|FindComponentbyTag _output_get "/Script/Engine.ShapeComponent" "Inventory"))
  (bind _ownersinvencollision (Variables|Default|GetOwnersInvenCollision)
    (:then
      (Collision|BindEventtoOnComponentBeginOverlap _ownersinvencollision (EventDispatchers|CreateEvent :!event Custom|CartCollisionOverlapStart))
      (Collision|BindEventtoOnComponentEndOverlap _ownersinvencollision (EventDispatchers|CreateEvent :!event Custom|CartCollisionOverlapEnd)))
    (:else)))