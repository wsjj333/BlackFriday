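; Replicated pawn component for two-handed item pickup, throwing and gun firing.
; Hold inputs send S_ events that sphere-trace at hand bones and attach a BP_ItemActor, tracked per hand; release detaches it with a hand-velocity impulse via SC_ItemDrop.
; While GunActive is set, fire input line-traces from the camera to aim the held gun.
; A BeginPlay RepNotify caches owner mesh and camera and adds the input mapping context.
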(event Custom|S_ItemPickUpAttach
  (params (PickUpHand :type Integer))
  ;[1 1 1] 아이템 픽업
  (CallFunction|ItemPickUpAttach PickUpHand))

(event Custom|S_GunFire
  (CallFunction|SCGunFire))

(event Custom|SC_ItemDrop
  (params (PickUpHand :type Integer) (Impulse :type Vector) (TargetLocation :type Vector))
  ;[1 1 1] 아이템 놓기/던지기
  (CallFunction|ItemDrop PickUpHand Impulse TargetLocation))

(event Custom|S_ItemDrop
  (params (PickUpHand :type Integer))
  ;[1 1 1] 아이템 놓기/던지기
  (bind (_handvelocity _targetlocation) (Class|BPHandVelocityInterface|GetHandVelocity(Message) (Variables|Default|GetOwnerPawn)))
  (CallFunction|SCItemDrop PickUpHand (Utilities|Array|Get(acopy) _handvelocity PickUpHand) (Utilities|Array|Get(acopy) _targetlocation PickUpHand)))

(event Custom|SC_GunFire
  (CallFunction|GunFire))

(event Custom|S_ItemPickUp
  (params (PickUpHand :type Integer))
  ;[1 1 1] 아이템 픽업
  (CallFunction|ItemPickUp PickUpHand "ForOneFrame" 8e+01))

(event Custom|SC_ItemPickUp
  (params (PickUpHand :type Integer))
  ;[1 1 1] 아이템 픽업
)

(event Input|EnhancedActionEvents|EnhancedInputActionIA_LeftHandHold
  (params (ActionValue :type Vector%202D%20Structure) (ElapsedSeconds :type Float%20%28double-precision%29) (TriggeredSeconds :type Float%20%28double-precision%29) (InputAction :type Input%20Action%20Object%20Reference :default "/Game/Colab/LEN/GunnerIMC/IA/IA_LeftHandHold.IA_LeftHandHold"))
  ;[1 1 1] 왼손 Item Attach
  (:Triggered
    (CallFunction|SItemPickUp))
  (:Completed
    (CallFunction|SItemDrop)))

(event Input|EnhancedActionEvents|EnhancedInputActionIA_RightHandHold
  (params (ActionValue :type Vector%202D%20Structure) (ElapsedSeconds :type Float%20%28double-precision%29) (TriggeredSeconds :type Float%20%28double-precision%29) (InputAction :type Input%20Action%20Object%20Reference :default "/Game/Colab/LEN/GunnerIMC/IA/IA_RightHandHold.IA_RightHandHold"))
  ;[1 1 1] 오른손 Item Attach
  (:Triggered
    (CallFunction|SItemPickUp 1))
  (:Completed
    (CallFunction|SItemDrop 1)))

(event Input|EnhancedActionEvents|EnhancedInputActionIA_GunFire
  (params (ActionValue :type Boolean) (ElapsedSeconds :type Float%20%28double-precision%29) (TriggeredSeconds :type Float%20%28double-precision%29) (InputAction :type Input%20Action%20Object%20Reference :default "/Game/Colab/LEN/GunnerIMC/IA/IA_GunFire.IA_GunFire"))
  ;[1 1 1] Gun Fire
  (:Started
    (CallFunction|SGunFire)))

(event EventBeginPlay
  (Variables|Default|SetbBeginPlay true))

(fn ItemPickUpAttach
  (params (PickUpHand :type Integer))
  (bind _output_get (LocalVariables|SetLFindItem (Utilities|Array|Get(acopy) (Variables|Default|GetAttachedItems) PickUpHand)))
  (LocalVariables|SetLActorScale (Transformation|GetActorScale3D _output_get))
  (bind _returnvalue (Transformation|AttachComponentToComponent (LocalVariables|GetLFindItem) (Variables|Default|GetOwnersSkeletalMesh) (Utilities|Array|Get(acopy) (Variables|Default|GetHandBones) PickUpHand) "SnapToTarget" "SnapToTarget" "SnapToTarget" false))
  (if _returnvalue
    (Default|SetAttachedItemSetting (LocalVariables|GetLFindItem) PickUpHand (LocalVariables|GetLActorScale))))

(fn ItemPickUp
  (params (PickUpHand :type Integer) (DrawDebugType :type EDrawDebugTrace%20Enum :default "None") (Radius :type Float%20%28single-precision%29))
  (bind _ownersskeletalmesh (Variables|Default|GetOwnersSkeletalMesh))
  (bind _handbones (Variables|Default|GetHandBones))
  (bind _output (Utilities|Array|Get(acopy) _handbones PickUpHand))
  (bind _returnvalue (Transformation|GetSocketLocation _ownersskeletalmesh _output))
  ;[1 1 1] 아이템이 붙여질 스켈레탈 메시가 필요
  (Utilities|IsValid (Variables|Default|GetOwnersSkeletalMesh)
    (:Is%20Valid
      (bind (_outhit _returnvalue_2) (Collision|SphereTraceByChannel _returnvalue _returnvalue Radius "TraceTypeQuery1" false 0 DrawDebugType true "(R=1.000000,G=0.000000,B=0.000000,A=1.000000)" "(R=0.000000,G=1.000000,B=0.000000,A=1.000000)" 1.0))
      (if _returnvalue_2
        (Utilities|IsValid (Utilities|Array|Get(acopy) (Variables|Default|GetAttachedItems) PickUpHand)
          (:Is%20Not%20Valid
            (bind _asbp_item_actor (Utilities|Casting|CastToBP_ItemActor (.HitActor (Collision|BreakHitResult _outhit))))
            (LocalVariables|SetLFind _asbp_item_actor)
            (if (and (not (Utilities|IsValid (Utilities|Array|Get(acopy) (Variables|Default|GetAttachedItems) PickUpHand))) (not (Utilities|Array|ContainsItem (Variables|Default|GetAttachedItems) (LocalVariables|GetLFind))))
              ;[1 1 1] 오너와 스켈레탈 메시가 있어야함
              (if (and (Utilities|IsValid (Variables|Default|GetOwnersSkeletalMesh)) (Utilities|IsValid (Variables|Default|GetOwnerPawn)))
                (Utilities|Array|SetArrayElem (Variables|Default|GetAttachedItems) PickUpHand (LocalVariables|GetLFind))
                (if (Utilities|Enum|Equal(Enum) (Variables|/Game/Colab/LEN/Item/BP_ItemActor.BP_ItemActor_C|GetAttackType (LocalVariables|GetLFind)) "NewEnumerator5")
                  (Variables|Default|SetGunActiveHand PickUpHand))
                (Default|SAttachHand (LocalVariables|GetLFind) (Variables|Default|GetOwnerPawn))
                (CallFunction|SItemPickUpAttach PickUpHand)))))))
    (:Is%20Not%20Valid
      (Development|PrintString "아이템을 붙일 스켈레탈 메시가 없습니다"))))

(fn ItemDrop
  (params (Hand :type Integer) (Impulse :type Vector) (TargetLocation :type Vector))
  (Utilities|IsValid (Utilities|Array|Get(acopy) (Variables|Default|GetAttachedItems) Hand)
    (:Is%20Valid
      (Development|PrintString "놓기")
      (Transformation|DetachFromActor (Utilities|Array|Get(acopy) (Variables|Default|GetAttachedItems) Hand) "KeepWorld" "KeepWorld" "KeepWorld")
      (Physics|SetSimulatePhysics (Variables|/Game/Colab/LEN/Item/BP_ItemActor.BP_ItemActor_C|GetStaticMesh (Utilities|Array|Get(acopy) (Variables|Default|GetAttachedItems) Hand)) true)
      ;[1 1 1] 속도를 받아와서 해당 방향으로 임팩트
      (Physics|AddImpulse (Variables|/Game/Colab/LEN/Item/BP_ItemActor.BP_ItemActor_C|GetStaticMesh (Utilities|Array|Get(acopy) (Variables|Default|GetAttachedItems) Hand)) Impulse "None" true)
      ;[1 1 1] 임팩트 방향 시각적 확인용
      (Collision|SphereTraceByChannel TargetLocation (+ TargetLocation (* Impulse 0.5)) 1e+01 "TraceTypeQuery1" false 0 "ForDuration")
      (Default|SDettachHand (Utilities|Array|Get(acopy) (Variables|Default|GetAttachedItems) Hand))
      ;[1 1 1] 배열에서 아이템지우기
      (Utilities|Array|SetArrayElem (Variables|Default|GetAttachedItems) Hand 0))))

(fn ActiveGun
  (Variables|Default|SetbGunActive true))

(fn NotActiveGun
  (Variables|Default|SetbGunActive false)
  (bind _crosshair (Variables|Default|GetCrossHair)
    (:then
      (Widget|RemovefromParent _crosshair))
    (:else)))

(fn GunFire
  (bind _ownerscamera (Variables|Default|GetOwnersCamera))
  (bind _returnvalue (Transformation|GetWorldLocation _ownerscamera))
  (if (Variables|Default|GetbGunActive)
    (bind _asbp_item_actor_gun_base (Utilities|Casting|CastToBP_ItemActor_GunBase (Utilities|Array|Get(acopy) (Variables|Default|GetAttachedItems) (Variables|Default|GetGunActiveHand))))
    (bind (_outhit _returnvalue_2) (Collision|LineTraceByChannel _returnvalue (+ _returnvalue (* (Math|Vector|GetForwardVector _ownerscamera) 5e+03)) "TraceTypeQuery1" false (Variables|Default|GetAttachedItems) "None"))
    (if _returnvalue_2
      (Default|GunFire _asbp_item_actor_gun_base (.Location (Collision|BreakHitResult _outhit)) true)
      (else
        (Default|GunFire _asbp_item_actor_gun_base (.TraceEnd (Collision|BreakHitResult _outhit)) false)))))

(fn SetMappingContext
  (bind _as플레이어_컨트롤러 (Utilities|Casting|CastToPlayerController (Pawn|GetController (Variables|Default|GetOwnerPawn))))
  (Utilities|IsValid (PlayerController|LocalPlayerSubsystems|GetEnhancedInputLocalPlayerSubsystem _as플레이어_컨트롤러)
    (:Is%20Valid
      (Input|AddMappingContext (PlayerController|LocalPlayerSubsystems|GetEnhancedInputLocalPlayerSubsystem _as플레이어_컨트롤러) "/Game/Colab/LEN/GunnerIMC/IMC_ItemPickUp.IMC_ItemPickUp" 0 "(bIgnoreAllPressedKeysUntilRelease=True,bForceImmediately=False,bNotifyUserSettings=False)"))))

(fn CustomBeginPlay
  (Class|ActorComponent|SetIsReplicated true)
  (bind _as폰 (Utilities|Casting|CastToPawn (Components|GetOwner)))
  (bind _output_get (Variables|Default|SetOwnerPawn _as폰))
  (Variables|Default|SetOwnersSkeletalMesh (Actor|GetComponentbyClass _output_get "/Script/Engine.SkeletalMeshComponent"))
  (Variables|Default|SetOwnersCamera (Actor|GetComponentbyClass (Variables|Default|GetOwnerPawn) "/Script/Engine.CameraComponent"))
  (CallFunction|SetMappingContext))

(fn OnRepBBeginPlay
  (CallFunction|CustomBeginPlay))