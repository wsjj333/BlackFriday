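; Pawn movement component that drives a physics-simulating root primitive with forces for walking and jumping.
; Move applies yaw-relative acceleration less horizontal velocity, clamps planar speed and turns the pawn toward its movement.
; S_MoveTick traces downward to set the falling state and ground normal, which projects grounded movement along slopes and gates the impulse jump.
; PhysicsMove duplicates the movement without rotation, but its only call sits in unreachable nodes.
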(event Custom|S_MoveTick
  (bind _ownersroot (Variables|Default|GetOwnersRoot))
  (bind _returnvalue (Transformation|GetWorldLocation _ownersroot))
  ;[1 1 1] 무브 틱
  (bind (_outhit _returnvalue_2) (Collision|LineTraceByChannel _returnvalue (- _returnvalue "0.000000,0.000000,100.000000") "TraceTypeQuery1" false 0 "ForOneFrame"))
  (if _returnvalue_2
    (Variables|Default|SetIsFalling false)
    ;;[1 1 1] 바닥 노말 받아오기
    (Variables|Default|SetGroundNormal (.Normal (Collision|BreakHitResult _outhit)))
    (else
      (Variables|Default|SetIsFalling true))))

(event Custom|Move
  (params (In%20Rot%20Z%20%28Yaw%29 :type Float%20%28single-precision%29) (X :type Float%20%28double-precision%29) (Y :type Float%20%28double-precision%29))
  (bind _returnvalue (Math|Vector|GetForwardVector (Math|Rotator|MakeRotator 0.0 0.0 In%20Rot%20Z%20%28Yaw%29)))
  (bind _returnvalue_2 (Math|Vector|GetRightVector (Math|Rotator|MakeRotator 0.0 0.0 In%20Rot%20Z%20%28Yaw%29)))
  (bind _ownerpawn (Variables|Default|GetOwnerPawn))
  (bind _returnvalue_3 (Transformation|GetVelocity _ownerpawn))
  (bind _returnvalue_4 (* _returnvalue_2 X))
  (bind _returnvalue_5 (* _returnvalue Y))
  (bind _returnvalue_6 (+ _returnvalue_4 _returnvalue_5))
  ;[1 1 1] 무브
  (if (Variables|Default|GetIsFalling)
    ;;[1 1 1] 공중에 떠있으면 그냥 움직이는 방향으로만
    (Variables|Default|SetMoveVar (* (Math|Vector|Normalize _returnvalue_6) 2e+03))
    (else
      ;;[1 1 1] 바닥에 있으면 바닥에영향
      (Variables|Default|SetMoveVar (* (Math|Vector|Normalize (Math|Vector|ProjectVectorontoPlane _returnvalue_6 (Variables|Default|GetGroundNormal))) 2e+03))))
  ;;[1 1 1] AddForce로 움직이기
  (Physics|AddForce (Variables|Default|GetOwnersRoot) (- (Variables|Default|GetMoveVar) (Math|Vector|MakeVector (.x _returnvalue_3) (.y _returnvalue_3) 0.0)) "None" true)
  ;;[1 1 1] 최대속도 제한
  (bind _returnvalue_7 (Physics|GetPhysicsLinearVelocity (Variables|Default|GetOwnersRoot) "None"))
  (Physics|SetPhysicsLinearVelocity (Variables|Default|GetOwnersRoot) (Math|Vector|VectorClampSize2D _returnvalue_7 -4e+02 4e+02) false "None")
  ;;[1 1 1] 움직이는 방향으로 캐릭터 로테이트
  (if (Variables|Default|GetIsMove)
    (Transformation|SetActorRotation (Variables|Default|GetOwnerPawn) (Math|Interpolation|RInterpTo (Transformation|GetActorRotation (Variables|Default|GetOwnerPawn)) (Math|Conversions|RotationFromXVector (Variables|Default|GetMoveVar)) (Utilities|Time|GetWorldDeltaSeconds) 1e+01) true)))

(event Custom|JumpServer
  ;[1 1 1] 점프로직
  (if (not (Variables|Default|GetIsFalling))
    (Physics|AddImpulse (Variables|Default|GetOwnersRoot) (Math|Vector|MakeVector 0.0 0.0 7e+02) "None" true)))

(event Custom|IsMoveing
  (params (IsMove :type Boolean))
  ;[1 1 1] IsMove On Off
  (Variables|Default|SetIsMove IsMove)
  (Variables|Default|SetMoveVar "0, 0, 0"))

(event EventBeginPlay
  (CallFunction|CustomBeginPlay))

(fn CustomBeginPlay
  (bind _as폰 (Utilities|Casting|CastToPawn (Components|GetOwner)))
  (bind _output_get (Variables|Default|SetOwnerPawn _as폰))
  (bind _as프리미티브_컴포넌트 (Utilities|Casting|CastToPrimitiveComponent (Variables|/Script/Engine.Actor|GetRootComponent _output_get)))
  (if (Class|SceneComponent|IsAnySimulatingPhysics _as프리미티브_컴포넌트)
    (Variables|Default|SetOwnersRoot _as프리미티브_컴포넌트)))

(fn PhysicsMove
  (params (InRotYaw :type Float%20%28single-precision%29) (X :type Float%20%28double-precision%29) (Y :type Float%20%28double-precision%29))
  (bind _returnvalue (Math|Vector|GetForwardVector (Math|Rotator|MakeRotator 0.0 0.0 InRotYaw)))
  (bind _returnvalue_2 (Math|Vector|GetRightVector (Math|Rotator|MakeRotator 0.0 0.0 InRotYaw)))
  (bind _ownerpawn (Variables|Default|GetOwnerPawn))
  (bind _returnvalue_3 (Transformation|GetVelocity _ownerpawn))
  (bind _returnvalue_4 (* _returnvalue_2 X))
  (bind _returnvalue_5 (* _returnvalue Y))
  (bind _returnvalue_6 (+ _returnvalue_4 _returnvalue_5))
  (Utilities|IsValid (Variables|Default|GetOwnersRoot)
    (:Is%20Valid
      (if (Variables|Default|GetIsFalling)
        ;[1 1 1] 공중에 떠있으면 그냥 움직이는 방향으로만
        (Variables|Default|SetMoveVar (* (Math|Vector|Normalize _returnvalue_6) 2e+03))
        (else
          ;[1 1 1] 바닥에 있으면 바닥에영향
          (Variables|Default|SetMoveVar (* (Math|Vector|Normalize (Math|Vector|ProjectVectorontoPlane _returnvalue_6 (Variables|Default|GetGroundNormal))) 2e+03))))
      ;[1 1 1] AddForce로 움직이기
      (Physics|AddForce (Variables|Default|GetOwnersRoot) (- (Variables|Default|GetMoveVar) (Math|Vector|MakeVector (.x _returnvalue_3) (.y _returnvalue_3) 0.0)) "None" true)
      ;[1 1 1] 최대속도 제한
      (bind _returnvalue_7 (Physics|GetPhysicsLinearVelocity (Variables|Default|GetOwnersRoot) "None"))
      (Physics|SetPhysicsLinearVelocity (Variables|Default|GetOwnersRoot) (Math|Vector|VectorClampSize2D _returnvalue_7 -4e+02 4e+02) false "None"))))