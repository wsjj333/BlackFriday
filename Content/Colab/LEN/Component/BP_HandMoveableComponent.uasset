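; Pawn component for mouse-driven, replicated control of a physically simulated character's left and right hands.
; Enhanced Input sends hold, mouse-delta and reach changes through server events, which compute clamped yaw and height targets around the pawn, plus hand velocity.
; RepNotified hold flags toggle physics below each arm bone and swap constraint profiles.
; An unfinished hand-fire path uses a camera trace and spawned target actor, but its trigger is unwired.
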(event Custom|PhBodyServer
  ;[1 1 1] 본 시뮬레이션
  (CallFunction|PhysicsBody))

(event Custom|Server_TraceDistance
  (params (Amount :type Float%20%28double-precision%29))
  ;[1 1 1] 팔 길이 늘리기
  (Variables|Default|SetTraceDistance (Math|Float|Clamp(Float) (+ Amount (Variables|Default|GetTraceDistance)) 0.0 5e+02)))

(event Custom|PhysicsBody
  (bind _returnvalue (Utilities|Name|MakeLiteralName "spine_01"))
  ;[1 1 1] 본 시뮬레이션
  (if (not (Physics|IsSimulatingPhysics (Variables|Default|GetOwnersSkeletalMesh) _returnvalue))
    (Class|SkeletalMeshComponent|SetAllBodiesBelowSimulatePhysics (Variables|Default|GetOwnersSkeletalMesh) _returnvalue true true)))

(event Custom|S_RightHandHoldStart
  (params (HandIndex :type Integer) (CameraForward :type Vector))
  ;[1 1 1] 팔 홀드 시작
  (CallFunction|HandMoveStart HandIndex CameraForward))

(event Custom|TickHandFire
  ;[1 1 1] 손 발사(미완성&불확실)
  (if (Variables|HandFire|GetbIsHandFire)
    (bind _targetactorsphereltest (Variables|HandFire|GetTargetActorSphereLTest)
      (:then
        (switch int (Variables|/Game/Colab/LEN/Character/GunnerPawnClassVer/BP_TargetActor.BP_TargetActor_C|GetIsMove _targetactorsphereltest)
          (:0
            (Variables|HandFire|SetbIsHandFire false)
            (Class|SkeletalMeshComponent|SetAllBodiesBelowSimulatePhysics (Variables|Default|GetOwnersSkeletalMesh) (Utilities|Array|Get(acopy) (Variables|Default|GetSimulateHandBones)) true false)
            (Class|SkeletalMeshComponent|SetConstraintProfile (Variables|Default|GetOwnersSkeletalMesh) (Utilities|Array|Get(acopy) (Variables|Default|GetProfileSettingBones)) "None" true))
          (:1
            (Utilities|Array|SetArrayElem (Variables|Default|GetTargetLocation) 0 (Transformation|GetActorLocation _targetactorsphereltest) :!label _label))
          (:2
            (goto _label))))
      (:else))))

(event Custom|PhBodyMul
  ;[1 1 1] 본 시뮬레이션
  (CallFunction|PhysicsBody))

(event Custom|S_RightHandHoldEnd
  (params (HandIndex :type Integer))
  ;[1 1 1] 팔 홀드 앤드
  (CallFunction|HandMoveEnd HandIndex))

(event Custom|S_OffsetHand
  (params (HandIndex :type Integer) (DeltaX :type Float%20%28double-precision%29) (DeltaY :type Float%20%28double-precision%29))
  ;[1 1 1] 팔 홀드 꾹
  (CallFunction|OffestHand HandIndex "None" DeltaX DeltaY))

(event Input|EnhancedActionEvents|EnhancedInputActionIA_LeftHandHold
  (params (ActionValue :type Vector%202D%20Structure) (ElapsedSeconds :type Float%20%28double-precision%29) (TriggeredSeconds :type Float%20%28double-precision%29) (InputAction :type Input%20Action%20Object%20Reference :default "/Game/Colab/LEN/GunnerIMC/IA/IA_LeftHandHold.IA_LeftHandHold"))
  ;[1 1 1] 왼손 Move
  (:Triggered
    (bind _playercontrollerref (Variables|Default|GetPlayerControllerRef)
      (:then
        (CallFunction|SOffsetHand 0 (.DeltaX (Class|PlayerController|GetInputMouseDelta _playercontrollerref)) (.DeltaY (Class|PlayerController|GetInputMouseDelta _playercontrollerref))))
      (:else)))
  (:Started
    (CallFunction|SRightHandHoldStart 0 (Math|Vector|GetForwardVector (Variables|Default|GetOwnersCamera))))
  (:Completed
    (CallFunction|SRightHandHoldEnd)))

(event Input|EnhancedActionEvents|EnhancedInputActionIA_HandDistanceUp
  (params (ActionValue :type Boolean) (ElapsedSeconds :type Float%20%28double-precision%29) (TriggeredSeconds :type Float%20%28double-precision%29) (InputAction :type Input%20Action%20Object%20Reference :default "/Game/Colab/LEN/GunnerIMC/IA/IA_HandDistanceUp.IA_HandDistanceUp"))
  ;[1 1 1] 팔 사거리 늘리기
  (:Started
    (CallFunction|ServerTraceDistance 1e+01)))

(event Input|EnhancedActionEvents|EnhancedInputActionIA_RightHandHold
  (params (ActionValue :type Vector%202D%20Structure) (ElapsedSeconds :type Float%20%28double-precision%29) (TriggeredSeconds :type Float%20%28double-precision%29) (InputAction :type Input%20Action%20Object%20Reference :default "/Game/Colab/LEN/GunnerIMC/IA/IA_RightHandHold.IA_RightHandHold"))
  ;[1 1 1] 오른손 Move
  (:Triggered
    (bind _playercontrollerref (Variables|Default|GetPlayerControllerRef)
      (:then
        (CallFunction|SOffsetHand 1 (.DeltaX (Class|PlayerController|GetInputMouseDelta _playercontrollerref)) (.DeltaY (Class|PlayerController|GetInputMouseDelta _playercontrollerref))))
      (:else)))
  (:Started
    (CallFunction|SRightHandHoldStart 1 (Math|Vector|GetForwardVector (Variables|Default|GetOwnersCamera))))
  (:Completed
    (CallFunction|SRightHandHoldEnd 1)))

(event Input|EnhancedActionEvents|EnhancedInputActionIA_HandDistanceDown
  (params (ActionValue :type Boolean) (ElapsedSeconds :type Float%20%28double-precision%29) (TriggeredSeconds :type Float%20%28double-precision%29) (InputAction :type Input%20Action%20Object%20Reference :default "/Game/Colab/LEN/GunnerIMC/IA/IA_HandDistanceDown.IA_HandDistanceDown"))
  ;[1 1 1] 팔 사거리 늘리기
  (:Started
    (CallFunction|ServerTraceDistance -1e+01)))

(event EventBeginPlay
  (CallFunction|CustomBeginPlay)
  (Variables|Default|SetbIsBeginPlay false)
  (bind _as플레이어_컨트롤러 (Utilities|Casting|CastToPlayerController (Pawn|GetController (Variables|Default|GetOwnerPawn))))
  (Variables|Default|SetPlayerControllerRef _as플레이어_컨트롤러)
  (Utilities|IsValid (PlayerController|LocalPlayerSubsystems|GetEnhancedInputLocalPlayerSubsystem _as플레이어_컨트롤러)
    (:Is%20Valid
      (Input|AddMappingContext (PlayerController|LocalPlayerSubsystems|GetEnhancedInputLocalPlayerSubsystem _as플레이어_컨트롤러) "/Game/Colab/LEN/GunnerIMC/IMC_HandMove.IMC_HandMove" 0 "(bIgnoreAllPressedKeysUntilRelease=True,bForceImmediately=False,bNotifyUserSettings=False)")
      (bind _returnvalue (Game|SpawnActorfromClass "/Game/Colab/LEN/Character/GunnerPawnClassVer/BP_TargetActor.BP_TargetActor_C" (Math|Transform|MakeTransform "0, 0, 0" "0, 0, 0" "1.000000,1.000000,1.000000") "Undefined" "MultiplyWithRoot" (Variables|Default|GetOwnerPawn) 0))
      (Variables|HandFire|SetTargetActorSphereLTest _returnvalue)
      ;[1 1 1] 카메라 컴포넌트 얻어오기
      (Variables|Default|SetOwnersCamera (Actor|GetComponentbyClass (Variables|Default|GetOwnerPawn) "/Script/Engine.CameraComponent")))))

(event Input|KeyboardEvents|DebugKeyQ
  (params (Key :type Key%20Structure :default "None") (ActionValue :type Input%20Action%20Value%20Structure))
  ;[1 1 1] 손 발사(미완성&불확실)
)

(fn SetHandMoveStart
  (params (Hand :type Integer))
  (Utilities|IsValid (Variables|Default|GetOwnersSkeletalMesh)
    (:Is%20Valid
      ;[1 1 1] 시뮬레이션 해제(upperarm)
      (Class|SkeletalMeshComponent|SetAllBodiesBelowSimulatePhysics (Variables|Default|GetOwnersSkeletalMesh) (Utilities|Array|Get(acopy) (Variables|Default|GetSimulateHandBones) Hand) false false)
      ;[1 1 1] 피직스 에셋에서 설정한 프로파일로 교체(lowerarm)
      (Class|SkeletalMeshComponent|SetConstraintProfile (Variables|Default|GetOwnersSkeletalMesh) (Utilities|Array|Get(acopy) (Variables|Default|GetProfileSettingBones) Hand) "New" true))))

(fn SetHandMoveEnd
  (params (Hand :type Integer))
  (Utilities|IsValid (Variables|Default|GetOwnersSkeletalMesh)
    (:Is%20Valid
      ;[1 1 1] 시뮬레이션 다시 활성화
      (Class|SkeletalMeshComponent|SetAllBodiesBelowSimulatePhysics (Variables|Default|GetOwnersSkeletalMesh) (Utilities|Array|Get(acopy) (Variables|Default|GetSimulateHandBones) Hand) true false)
      ;[1 1 1] 프로파일을 다시 원래 셋팅으로
      (Class|SkeletalMeshComponent|SetConstraintProfile (Variables|Default|GetOwnersSkeletalMesh) (Utilities|Array|Get(acopy) (Variables|Default|GetProfileSettingBones) Hand) "None" true))))

(fn HandMoveStart
  (params (Hand :type Integer) (CameraForward :type Vector))
  (if (and (Utilities|IsValid (Variables|Default|GetOwnerPawn)) (Utilities|IsValid (Variables|Default|GetOwnersSkeletalMesh)))
    (LocalVariables|SetLSelectHandBone (Utilities|Array|Get(acopy) (Variables|Default|GetHandBones) Hand))
    ;[1 1 1] 초기 시작점 설정
    (LocalVariables|SetLStartLocation (+ (Transformation|GetActorLocation (Variables|Default|GetOwnerPawn)) (* CameraForward 2e+02)))
    ;[1 1 1] TargetLocation
    (Utilities|Array|SetArrayElem (Variables|Default|GetTargetLocation) Hand (Transformation|GetSocketLocation (Variables|Default|GetOwnersSkeletalMesh) (LocalVariables|GetLSelectHandBone)))
    ;[1 1 1] 시작점의 각도와 높이 저장
    (Utilities|Array|SetArrayElem (Variables|Default|GetCurrentAngle) (LocalVariables|Gethand) (Math|Float|Clamp(Float) (.yaw (Math|Rotator|Delta(Rotator) (Math|Rotator|FindLookatRotation (Transformation|GetActorLocation (Variables|Default|GetOwnerPawn)) (LocalVariables|GetLStartLocation)) (Transformation|GetActorRotation (Variables|Default|GetOwnerPawn)))) (Utilities|Array|Get(acopy) (Variables|Default|GetMinAngle) (LocalVariables|Gethand)) (Utilities|Array|Get(acopy) (Variables|Default|GetMaxAngle) (LocalVariables|Gethand))))
    (Utilities|Array|SetArrayElem (Variables|Default|GetCurrHeight) (LocalVariables|Gethand) (+ (.Z (Math|Vector|BreakVector (- (LocalVariables|GetLStartLocation) (Transformation|GetActorLocation (Variables|Default|GetOwnerPawn))))) 5e+01))
    (switch int Hand
      (:0
        (Variables|Default|SetLeftHandHold true))
      (:1
        (Variables|Default|SetRightHandHold true)))))

(fn HandMoveEnd
  (params (Hand :type Integer))
  (switch int Hand
    (:0
      (Variables|Default|SetLeftHandHold false))
    (:1
      (Variables|Default|SetRightHandHold false))))

(fn OffestHand
  (params (hand :type Integer) (DrawDebugType :type EDrawDebugTrace%20Enum :default "None") (DeltaX :type Float%20%28double-precision%29) (DeltaY :type Float%20%28double-precision%29))
  (bind _currheight (Variables|Default|GetCurrHeight))
  (bind _ownerpawn (Variables|Default|GetOwnerPawn))
  (bind _ownerpawn_2 (Variables|Default|GetOwnerPawn))
  (bind _currentangle (Variables|Default|GetCurrentAngle))
  (bind _tracedistance (Variables|Default|GetTraceDistance))
  (bind _returnvalue (Transformation|GetActorRotation _ownerpawn_2))
  (bind _returnvalue_2 (Transformation|GetActorLocation _ownerpawn))
  (bind _output (Utilities|Array|Get(acopy) _currentangle hand))
  (bind _output_2 (Utilities|Array|Get(acopy) _currheight hand))
  (bind _returnvalue_3 (Math|Vector|MakeVector 0.0 0.0 _output_2))
  (bind (_roll _pitch _yaw) (Math|Rotator|BreakRotator _returnvalue))
  (bind _returnvalue_4 (+ _yaw _output))
  (bind _returnvalue_5 (Math|Rotator|MakeRotator _roll _pitch _returnvalue_4))
  (bind _returnvalue_6 (Math|Vector|GetForwardVector _returnvalue_5))
  (bind _returnvalue_7 (* _returnvalue_6 _tracedistance))
  (bind _returnvalue_8 (+ _returnvalue_2 _returnvalue_7))
  (bind _returnvalue_9 (+ _returnvalue_8 _returnvalue_3))
  (Utilities|IsValid (Variables|Default|GetOwnerPawn)
    (:Is%20Valid
      ;[1 1 1] 계산된 각도
      (Utilities|Array|SetArrayElem (Variables|Default|GetCurrentAngle) hand (Math|Float|Clamp(Float) (+ (* DeltaX (Variables|Default|GetSensitivityX)) (Utilities|Array|Get(acopy) (Variables|Default|GetCurrentAngle) hand)) (Utilities|Array|Get(acopy) (Variables|Default|GetMinAngle) hand) (Utilities|Array|Get(acopy) (Variables|Default|GetMaxAngle) hand)))
      ;[1 1 1] 계산된 높이
      (Utilities|Array|SetArrayElem (Variables|Default|GetCurrHeight) hand (Math|Float|Clamp(Float) (+ (* DeltaY (Variables|Default|GetSensitivityY)) (Utilities|Array|Get(acopy) (Variables|Default|GetCurrHeight) hand)) (Variables|Default|GetMinHeight) (Variables|Default|GetMaxHeight)))
      ;[1 1 1] 손의 최종위치
      (Utilities|Array|SetArrayElem (Variables|Default|GetTargetLocation) hand _returnvalue_9)
      ;[1 1 1] 현제 속도 계산
      (Utilities|Array|SetArrayElem (Variables|Default|GetHandVelocity) hand (/ (- (Utilities|Array|Get(acopy) (Variables|Default|GetTargetLocation) hand) (Utilities|Array|Get(acopy) (Variables|Default|GetBeforeTargetLocation) hand)) (Utilities|Time|GetWorldDeltaSeconds)))
      ;[1 1 1] 이전 벡터 갱신
      (Utilities|Array|SetArrayElem (Variables|Default|GetBeforeTargetLocation) hand (Utilities|Array|Get(acopy) (Variables|Default|GetTargetLocation) hand))
      ;[1 1 1] 디버그 (최종 위치확인용)
      (Collision|SphereTraceByChannel _returnvalue_9 _returnvalue_9 1e+01 "TraceTypeQuery1" false 0 DrawDebugType))))

(fn SetPhysicsConstraint
  (for _index (range 0 1)
    (bind _returnvalue (Game|AddComponentbyClass (Variables|Default|GetOwnerPawn) "/Script/Engine.PhysicsConstraintComponent" false))
    (Utilities|Array|Add (Variables|Default|GetPhysicsConstraints) _returnvalue)
    (Transformation|AttachComponentToComponent _returnvalue (Variables|Default|GetOwnersSkeletalMesh) (Utilities|Array|Get(acopy) (Variables|Default|GetHandBones) _index) "SnapToTarget" "SnapToTarget" "KeepRelative" true)))

(fn OnRepLeftHandHold
  (if (Variables|Default|GetLeftHandHold)
    (CallFunction|SetHandMoveStart)
    (else
      (CallFunction|SetHandMoveEnd))))

(fn OnRepRightHandHold
  (if (Variables|Default|GetRightHandHold)
    (CallFunction|SetHandMoveStart 1)
    (else
      (CallFunction|SetHandMoveEnd 1))))

(fn CustomBeginPlay
  (bind _as폰 (Utilities|Casting|CastToPawn (Components|GetOwner)))
  (bind _output_get (Variables|Default|SetOwnerPawn _as폰))
  (Variables|Default|SetOwnersSkeletalMesh (Actor|GetComponentbyClass _output_get "/Script/Engine.SkeletalMeshComponent"))
  (CallFunction|SetPhysicsConstraint))

(fn OnRepBIsBeginPlay
  (CallFunction|CustomBeginPlay)
  (Utilities|FlowControl|Sequence
    (:then_0
      (if (Variables|Default|GetLeftHandHold)
        (CallFunction|SetHandMoveStart)
        (else
          (CallFunction|SetHandMoveEnd))))
    (:then_1
      (if (Variables|Default|GetRightHandHold)
        (CallFunction|SetHandMoveStart 1)
        (else
          (CallFunction|SetHandMoveEnd 1))))))

(fn OnRepIsSimulate
  (if (Variables|Default|GetIsSimulate)
    (CallFunction|PhysicsBody)
    (CallFunction|PhBodyServer)))

(fn ShootHand
  (bind _ownerscamera (Variables|Default|GetOwnersCamera))
  (bind _returnvalue (Transformation|GetWorldLocation _ownerscamera))
  (bind (_outhit _returnvalue_2) (Collision|LineTraceByChannel _returnvalue (+ _returnvalue (* (Math|Vector|GetForwardVector _ownerscamera) 1.3e+03)) "TraceTypeQuery1" false 0 "ForDuration"))
  (if _returnvalue_2
    (Variables|HandFire|SetHandFireLocation (.ImpactPoint (Collision|BreakHitResult _outhit)))
    (else
      (Variables|HandFire|SetHandFireLocation (.TraceEnd (Collision|BreakHitResult _outhit)))))
  (bind _targetactorsphereltest (Variables|HandFire|GetTargetActorSphereLTest)
    (:then
      ;[1 1 1] 시뮬레이션 해제(upperarm)
      (Class|SkeletalMeshComponent|SetAllBodiesBelowSimulatePhysics (Variables|Default|GetOwnersSkeletalMesh) (Utilities|Array|Get(acopy) (Variables|Default|GetSimulateHandBones)) false false)
      ;[1 1 1] 피직스 에셋에서 설정한 프로파일로 교체(lowerarm)
      (Class|SkeletalMeshComponent|SetConstraintProfile (Variables|Default|GetOwnersSkeletalMesh) (Utilities|Array|Get(acopy) (Variables|Default|GetProfileSettingBones)) "New" true)
      (Default|SetMove _targetactorsphereltest (Variables|HandFire|GetHandFireLocation) (Transformation|GetActorLocation (Variables|Default|GetOwnerPawn))))
    (:else)))