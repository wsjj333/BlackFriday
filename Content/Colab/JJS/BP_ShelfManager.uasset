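; Shelf manager actor that lays out a grid of instanced shelf meshes and stocks it with random items.
; The construction script adds one mesh instance per cell from row, column and spacing variables.
; BeginPlay repeats the grid math in the actor's transform, spawning a random ItemClasses entry slightly above each cell, without inheriting actor rotation.
; Disconnected alternatives using ShelfTransforms or a single-row layout never run.
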(event EventBeginPlay
  (for _index (range 0 (- (Variables|Default|GetRoxCount) 1))
    (for _index_2 (range 0 (- (Variables|Default|GetColumnCount) 1))
      (Game|SpawnActorfromClass (.OutItem (Utilities|Array|Random (Variables|Default|GetItemClasses))) (Math|Conversions|ToTransform(Vector) (+ (Math|Transform|TransformLocation (Transformation|GetActorTransform) (Math|Vector|MakeVector (* _index_2 (Variables|Default|GetSpacingX)) (* _index (Variables|Default|GetSpacingY)) 0.0)) "0.000000,0.000000,100.000000")) "AlwaysSpawn" "MultiplyWithRoot" 0 "NewEnumerator0" 0))))

(event Collision|EventActorBeginOverlap
  (params (OtherActor :type Actor%20Object%20Reference)))

(event EventTick
  (params (DeltaSeconds :type Float%20%28single-precision%29)))

(fn ConstructionScript
  (for _index (range 0 (- (Variables|Default|GetRoxCount) 1))
    (for _index_2 (range 0 (- (Variables|Default|GetColumnCount) 1))
      (Components|InstancedStaticMesh|AddInstance (Variables|Default|GetInstancedStaticMesh) (Math|Transform|MakeTransform (Math|Vector|MakeVector (* _index_2 (Variables|Default|GetSpacingX)) (* _index (Variables|Default|GetSpacingY)) 0.0)) false))))