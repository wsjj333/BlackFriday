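; BP_GoalCounter is a goal trigger that counts arrivals and raises a mesh once the third is registered.
; Each Box begin overlap increments ArrivedTeams, with no check on the overlapping actor and no decrement on exit.
; When the count equals three, a DoOnce plays a Timeline that lerps the StaticMesh upward along relative Z, keeping its X and Y.
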(event OnComponentBeginOverlap(Box)
  (params (OverlappedComponent :type Primitive%20Component%20Object%20Reference) (OtherActor :type Actor%20Object%20Reference) (OtherComp :type Primitive%20Component%20Object%20Reference) (OtherBodyIndex :type Integer) (bFromSweep :type Boolean) (SweepResult :type Hit%20Result%20Structure%20%28by%20ref%29))
  (bind _staticmesh (Variables|Default|GetStaticMesh))
  (bind _relativelocation (Variables|/Script/Engine.SceneComponent|GetRelativeLocation _staticmesh))
  (bind _result (Math|Integer|IncrementInt (Variables|Default|GetArrivedTeams))
    (:%20%20
      (if (== _result 3)
        (Utilities|FlowControl|DoOnce false
          (:Completed
            (bind _alpha (Timeline|Timeline PlayFromStart)
              (:Update
                (Transformation|SetRelativeLocation (Variables|Default|GetStaticMesh) (Math|Vector|Lerp(Vector) (Math|Vector|MakeVector (.x _relativelocation) (.y _relativelocation) -4e+02) (Math|Vector|MakeVector (.x _relativelocation) (.y _relativelocation) 1e+01) _alpha) false false)))))))))

(event EventBeginPlay)

(event Collision|EventActorBeginOverlap
  (params (OtherActor :type Actor%20Object%20Reference)))

(event EventTick
  (params (DeltaSeconds :type Float%20%28single-precision%29)))

(fn ConstructionScript)