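; BP_CartTest is a test physics cart driven by forces on a Box component, using Enhanced Input.
; Each tick, four wheel line traces apply spring-like suspension forces scaled by compression.
; Smoothed throttle input, decaying toward zero, drives forward force, shifts center of mass along X and scales steering torque.
; The computed Acceleration value is not used by the drive force, which reads AccelerationInput directly.
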(event Input|EnhancedActionEvents|EnhancedInputActionIA_Acceleration
  (params (ActionValue :type Float%20%28double-precision%29) (ElapsedSeconds :type Float%20%28double-precision%29) (TriggeredSeconds :type Float%20%28double-precision%29) (InputAction :type Input%20Action%20Object%20Reference :default "/Game/Colab/CCW/Cart/Input/Actions/IA_Acceleration.IA_Acceleration"))
  ;[1 1 1] 가속 키 눌렀을 때
  (Variables|Default|SetAccelerationInput (Math|Interpolation|FInterpTo (Variables|Default|GetAccelerationInput) ActionValue (Utilities|Time|GetWorldDeltaSeconds) 0.5)))

(event Input|EnhancedActionEvents|EnhancedInputActionIA_Steer
  (params (ActionValue :type Float%20%28double-precision%29) (ElapsedSeconds :type Float%20%28double-precision%29) (TriggeredSeconds :type Float%20%28double-precision%29) (InputAction :type Input%20Action%20Object%20Reference :default "/Game/Colab/CCW/Cart/Input/Actions/IA_Steer.IA_Steer"))
  (:Triggered
    (Class|PrimitiveComponent|AddTorqueinRadians (Variables|Default|GetBox) (Math|Vector|MakeVector 0.0 0.0 (* ActionValue 9e+07 (Variables|Default|GetAccelerationInput))) "None" false)))

(event EventBeginPlay
  ;[1 1 1] 초기화
  (Input|AddMappingContext (PlayerController|LocalPlayerSubsystems|GetEnhancedInputLocalPlayerSubsystem (Game|GetPlayerController 0)) "/Game/Colab/CCW/Cart/Input/IMC_CartTest.IMC_CartTest" 0 "(bIgnoreAllPressedKeysUntilRelease=True,bForceImmediately=False,bNotifyUserSettings=False)"))

(event EventTick
  (params (DeltaSeconds :type Float%20%28single-precision%29))
  ;[1 1 1] 매 프레임 실행
  (CallFunction|SuspensionCast (Variables|Default|GetFLWheel))
  (CallFunction|SuspensionCast (Variables|Default|GetFRWheel))
  (CallFunction|SuspensionCast (Variables|Default|GetBLWheel))
  (CallFunction|SuspensionCast (Variables|Default|GetBRWheel))
  (CallFunction|AddAcceleration)
  (CallFunction|CalculateAcceleration))

(fn ConstructionScript)

(fn SuspensionCast
  (params (WheelComp :type Scene%20Component%20Object%20Reference))
  (bind _returnvalue (Transformation|GetWorldLocation WheelComp))
  (bind _outhit (Collision|LineTraceByChannel _returnvalue (+ _returnvalue (* (Math|Vector|GetUpVector WheelComp) -6e+01)) "TraceTypeQuery1" false 0 "ForOneFrame"))
  (if (.bBlockingHit (Collision|BreakHitResult _outhit))
    (Class|PrimitiveComponent|AddForceatLocation (Variables|Default|GetBox) (* (- 1.0 (Math|Float|NormalizetoRange (.Distance (Collision|BreakHitResult _outhit)) 0.0 6e+01)) (Math|Vector|GetUnitDirection(Vector) (.TraceEnd (Collision|BreakHitResult _outhit)) (.TraceStart (Collision|BreakHitResult _outhit))) 1e+07) (Transformation|GetWorldLocation WheelComp) "None") ; Target(카트)의 벡터에\nLocation(Wheel Comp)를 힘의 작용점으로 해서\nForce(압축율 + 위쪽 방향) 벡터를 더한다\n즉, 서스펜션이 압축된 만큼 다시 위쪽으로 카트를 들어올린다
  ))

(fn CalculateAcceleration
  (Variables|Default|SetAcceleration (* (Math|Float|Lerp 0.0 1.5e+04 (Variables|Default|GetAccelerationInput)) (Variables|Default|GetAccelerationInput)))
  (Variables|Default|SetAccelerationInput (Math|Interpolation|FInterpTo (Variables|Default|GetAccelerationInput) 0.0 (Utilities|Time|GetWorldDeltaSeconds) 0.3)))

(fn AddAcceleration
  (bind _box (Variables|Default|GetBox))
  (Class|PrimitiveComponent|AddForceatLocation _box (* (Math|Vector|GetForwardVector _box) (Variables|Default|GetAccelerationInput) 1e+04 (Physics|GetMass _box)) (Transformation|GetWorldLocation _box) "None")
  (CallFunction|AddEffecttoCart))

(fn AddEffecttoCart
  (Class|PrimitiveComponent|SetCenterOfMass (Variables|Default|GetBox) (* "100.000000,0.000000,0.000000" (Variables|Default|GetAccelerationInput)) "None"))